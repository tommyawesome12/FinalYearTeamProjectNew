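; BP_FogGlich is a trigger Blueprint that reveals fog when the player enters one of its boxes.
; Three box components share one overlap response, which checks for the Player tag, prints a debug message and makes the FogBox0 component of the referenced FogCircle visible.
; The fog is only ever shown, as nothing here hides it again.
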(event OnComponentBeginOverlap(Box)
  (params (OverlappedComponent :type Primitive%20Component%20Object%20Reference) (OtherActor :type Actor%20Object%20Reference) (OtherComp :type Primitive%20Component%20Object%20Reference) (OtherBodyIndex :type Integer) (bFromSweep :type Boolean) (SweepResult :type Hit%20Result%20Structure%20%28by%20ref%29))
  (if (Actor|ActorHasTag OtherActor "Player")
    (Development|PrintText "Hello")
    (Rendering|SetVisibility (Variables|/Game/Sharan/Blueprints/BP_FogCircle.BP_FogCircle_C|GetFogBox_0 (Variables|Default|GetFogCircle)) true false)))

(event OnComponentBeginOverlap(Box1)
  (params (OverlappedComponent :type Primitive%20Component%20Object%20Reference) (OtherActor :type Actor%20Object%20Reference) (OtherComp :type Primitive%20Component%20Object%20Reference) (OtherBodyIndex :type Integer) (bFromSweep :type Boolean) (SweepResult :type Hit%20Result%20Structure%20%28by%20ref%29))
  (if (Actor|ActorHasTag OtherActor "Player")
    (Development|PrintText "Hello")
    (Rendering|SetVisibility (Variables|/Game/Sharan/Blueprints/BP_FogCircle.BP_FogCircle_C|GetFogBox_0 (Variables|Default|GetFogCircle)) true false)))

(event OnComponentBeginOverlap(Box2)
  (params (OverlappedComponent :type Primitive%20Component%20Object%20Reference) (OtherActor :type Actor%20Object%20Reference) (OtherComp :type Primitive%20Component%20Object%20Reference) (OtherBodyIndex :type Integer) (bFromSweep :type Boolean) (SweepResult :type Hit%20Result%20Structure%20%28by%20ref%29))
  (if (Actor|ActorHasTag OtherActor "Player")
    (Development|PrintText "Hello")
    (Rendering|SetVisibility (Variables|/Game/Sharan/Blueprints/BP_FogCircle.BP_FogCircle_C|GetFogBox_0 (Variables|Default|GetFogCircle)) true false)))

(fn ConstructionScript)