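; Roof crumbling effect that shows falling ceiling dust and plays audio when a low-sanity player is inside its trigger box.
; Box overlaps with Player-tagged actors toggle the JustWork flag, while Tick polls the player character's Sanity against a threshold.
; A DoOnce gate limits the dust reveal and audio component creation, re-arming on box entry or higher sanity.
; Leaving the box or regaining sanity hides the dust and stops the audio.
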(event OnComponentBeginOverlap(Box)
  (params (OverlappedComponent :type Primitive%20Component%20Object%20Reference) (OtherActor :type Actor%20Object%20Reference) (OtherComp :type Primitive%20Component%20Object%20Reference) (OtherBodyIndex :type Integer) (bFromSweep :type Boolean) (SweepResult :type Hit%20Result%20Structure%20%28by%20ref%29))
  (if (Actor|ActorHasTag OtherActor "Player")
    (Variables|Default|SetJustWork true)
    (Utilities|FlowControl|DoOnce false) ; enters at Reset
  ))

(event OnComponentEndOverlap(Box)
  (params (OverlappedComponent :type Primitive%20Component%20Object%20Reference) (OtherActor :type Actor%20Object%20Reference) (OtherComp :type Primitive%20Component%20Object%20Reference) (OtherBodyIndex :type Integer))
  (if (Actor|ActorHasTag OtherActor "Player")
    (Variables|Default|SetJustWork false)))

(event EventBeginPlay
  (Rendering|SetVisibility (Variables|Default|GetCeilingDust2) false false)
  (bind _asbp_player_character (Utilities|Casting|CastToBP_PlayerCharacter (Game|GetPlayerCharacter 0)))
  (Variables|Default|SetAs%20BP%20Player%20Character _asbp_player_character))

(event EventTick
  (params (DeltaSeconds :type Float%20%28single-precision%29))
  (Utilities|FlowControl|Sequence
    (:then_0
      (if (Variables|Default|GetJustWork)
        (Utilities|FlowControl|DoOnce false :!label _label
          (:Completed
            (if (Variables|Default|GetJustWork)
              (if (< (Variables|/Game/Tom/Tom_Blueprints/BP_PlayerCharacter.BP_PlayerCharacter_C|GetSanity (Variables|Default|GetAs%20BP%20Player%20Character)) 0.3)
                (Rendering|SetVisibility (Variables|Default|GetCeilingDust2) true false)
                (bind _returnvalue (AddComponent|AddAudioComponent (Variables|Default|GetAs%20BP%20Player%20Character) false))))))
        (else
          (Rendering|SetVisibility (Variables|Default|GetCeilingDust2) false false :!label _label_2)
          (Utilities|IsValid _returnvalue
            (:Is%20Valid
              (Audio|Components|Audio|Stop _returnvalue))))))
    (:then_1
      (if (> (Variables|/Game/Tom/Tom_Blueprints/BP_PlayerCharacter.BP_PlayerCharacter_C|GetSanity (Variables|Default|GetAs%20BP%20Player%20Character)) 0.3)
        (Utilities|FlowControl|Sequence
          (:then_0
            (goto _label Reset))
          (:then_1
            (goto _label_2)))))))

(fn ConstructionScript)