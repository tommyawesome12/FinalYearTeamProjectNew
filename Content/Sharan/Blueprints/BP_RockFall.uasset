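; BP_RockFall is an actor that plays a Niagara effect, presumably falling rocks, when the player character's Sanity drops between 0.1 and 0.25.
; Tick polls Sanity on the player reference cached at BeginPlay and fires through a DoOnce, which re-arms once Sanity rises above 0.3.
; Each trigger waits a random delay, spawns the effect at random scale, then destroys it after another random delay.
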(event EventBeginPlay
  (bind _asbp_player_character (Utilities|Casting|CastToBP_PlayerCharacter (Game|GetPlayerCharacter 0)))
  (Variables|Default|SetAs%20BP%20Player%20Character _asbp_player_character))

(event EventTick
  (params (DeltaSeconds :type Float%20%28single-precision%29))
  (bind _returnvalue (Math|Random|RandomFloatinRange 0.7 4.5))
  (bind _as_bp_player_character (Variables|Default|GetAs%20BP%20Player%20Character))
  (bind _as_bp_player_character_2 (Variables|Default|GetAs%20BP%20Player%20Character))
  (bind _sanity (Variables|/Game/Tom/Tom_Blueprints/BP_PlayerCharacter.BP_PlayerCharacter_C|GetSanity _as_bp_player_character))
  (bind _sanity_2 (Variables|/Game/Tom/Tom_Blueprints/BP_PlayerCharacter.BP_PlayerCharacter_C|GetSanity _as_bp_player_character_2))
  (Utilities|FlowControl|Sequence
    (:then_0
      (if (and (< _sanity_2 0.25) (> _sanity_2 0.1))
        (Utilities|FlowControl|DoOnce false :!label _label
          (:Completed
            (if (and (< _sanity 0.25) (> _sanity 0.1))
              (Utilities|FlowControl|Delay (Math|Random|RandomFloatinRange 0.2 4.0))
              (bind _returnvalue_2 (AddComponent|AddNiagaraComponent false (Math|Transform|MakeTransform "0, 0, 0" "0, 0, 0" (Math|Vector|MakeVector _returnvalue _returnvalue (Math|Random|RandomFloatinRange 0.7 2.0)))))
              (Utilities|FlowControl|Delay (Math|Random|RandomFloatinRange 9.0 15.0))
              (Components|DestroyComponent _returnvalue_2))))))
    (:then_1
      (if (> (Variables|/Game/Tom/Tom_Blueprints/BP_PlayerCharacter.BP_PlayerCharacter_C|GetSanity (Variables|Default|GetAs%20BP%20Player%20Character)) 0.3)
        (goto _label Reset)))))

(fn ConstructionScript)