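; Trigger-volume actor that thickens fog in steps as the player moves through numbered zones.
; BeginPlay creates dynamic fog and outline materials, puts the outline into the player's post-process blendables and hides the fog box.
; The Outline volume shows the fog, zeroes outline thickness and blocks the player's fade to black, reversing these on exit.
; Zones 1–5 raise or lower fog intensity; light-flicker logic is left disconnected.
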(event OnComponentBeginOverlap(Outline)
  (params (OverlappedComponent :type Primitive%20Component%20Object%20Reference) (OtherActor :type Actor%20Object%20Reference) (OtherComp :type Primitive%20Component%20Object%20Reference) (OtherBodyIndex :type Integer) (bFromSweep :type Boolean) (SweepResult :type Hit%20Result%20Structure%20%28by%20ref%29))
  (if (Actor|ActorHasTag OtherActor "Player")
    (Utilities|FlowControl|Sequence
      (:then_0
        (Rendering|Material|SetScalarParameterValue (Variables|Default|GetOutlineShaderMaterial) "Thickness NO" 0.0 :!class /Script/Engine.MaterialInstanceDynamic)
        (Rendering|Material|SetScalarParameterValue (Variables|Default|GetOutlineShaderMaterial) "Thickness DO" 0.0 :!class /Script/Engine.MaterialInstanceDynamic))
      (:then_1
        (Rendering|SetVisibility (Variables|/Game/Sharan/Blueprints/BP_Fog.BP_Fog_C|GetCube (Variables|Default|GetFogBox)) true false)
        (Rendering|Material|SetScalarParameterValue (Variables|Default|GetFogMaterial) "Intensity" 0.1 :!class /Script/Engine.MaterialInstanceDynamic)
        (bind _returnvalue (Rendering|Material|CreateDynamicMaterialInstance "/Game/Sharan/Materials/M_LightFlicker.M_LightFlicker" "None" "None" :!class /Script/Engine.KismetMaterialLibrary)))
      (:then_2
        (Variables|/Game/Tom/Tom_Blueprints/BP_PlayerCharacter.BP_PlayerCharacter_C|SetCanFadeToBlack (Variables|Default|GetAs%20BP%20Player%20Character) false)))))

(event OnComponentBeginOverlap(1)
  (params (OverlappedComponent :type Primitive%20Component%20Object%20Reference) (OtherActor :type Actor%20Object%20Reference) (OtherComp :type Primitive%20Component%20Object%20Reference) (OtherBodyIndex :type Integer) (bFromSweep :type Boolean) (SweepResult :type Hit%20Result%20Structure%20%28by%20ref%29))
  (if (Actor|ActorHasTag OtherActor "Player")
    (Rendering|Material|SetScalarParameterValue (Variables|Default|GetFogMaterial) "Intensity" 0.2 :!class /Script/Engine.MaterialInstanceDynamic)))

(event OnComponentEndOverlap(5)
  (params (OverlappedComponent :type Primitive%20Component%20Object%20Reference) (OtherActor :type Actor%20Object%20Reference) (OtherComp :type Primitive%20Component%20Object%20Reference) (OtherBodyIndex :type Integer))
  (if (Actor|ActorHasTag OtherActor "Player")
    (Rendering|Material|SetScalarParameterValue (Variables|Default|GetFogMaterial) "Intensity" 0.8 :!class /Script/Engine.MaterialInstanceDynamic)))

(event OnComponentEndOverlap(Outline)
  (params (OverlappedComponent :type Primitive%20Component%20Object%20Reference) (OtherActor :type Actor%20Object%20Reference) (OtherComp :type Primitive%20Component%20Object%20Reference) (OtherBodyIndex :type Integer))
  (if (Actor|ActorHasTag OtherActor "Player")
    (Utilities|FlowControl|Sequence
      (:then_0
        (Rendering|Material|SetScalarParameterValue (Variables|Default|GetOutlineShaderMaterial) "Thickness NO" 1.6 :!class /Script/Engine.MaterialInstanceDynamic)
        (Rendering|Material|SetScalarParameterValue (Variables|Default|GetOutlineShaderMaterial) "Thickness DO" 2.0 :!class /Script/Engine.MaterialInstanceDynamic))
      (:then_1
        (Rendering|SetVisibility (Variables|/Game/Sharan/Blueprints/BP_Fog.BP_Fog_C|GetCube (Variables|Default|GetFogBox)) false false)
        (bind _returnvalue (Rendering|Material|CreateDynamicMaterialInstance 0 "None" "None" :!class /Script/Engine.KismetMaterialLibrary)))
      (:then_2
        (Variables|/Game/Tom/Tom_Blueprints/BP_PlayerCharacter.BP_PlayerCharacter_C|SetCanFadeToBlack (Variables|Default|GetAs%20BP%20Player%20Character) true)))))

(event OnComponentBeginOverlap(ShaderTrigger)
  (params (OverlappedComponent :type Primitive%20Component%20Object%20Reference) (OtherActor :type Actor%20Object%20Reference) (OtherComp :type Primitive%20Component%20Object%20Reference) (OtherBodyIndex :type Integer) (bFromSweep :type Boolean) (SweepResult :type Hit%20Result%20Structure%20%28by%20ref%29))
  (if (Actor|ActorHasTag OtherActor "Player")
    (Utilities|FlowControl|Gate true ; enters at Open
      (:Exit
        (CallFunction|UpdateShader)))))

(event OnComponentEndOverlap(ShaderTrigger)
  (params (OverlappedComponent :type Primitive%20Component%20Object%20Reference) (OtherActor :type Actor%20Object%20Reference) (OtherComp :type Primitive%20Component%20Object%20Reference) (OtherBodyIndex :type Integer))
  (if (Actor|ActorHasTag OtherActor "Player")
    (Utilities|FlowControl|Gate true ; enters at Close
      (:Exit
        (CallFunction|UpdateShader)))))

(event OnComponentBeginOverlap(2)
  (params (OverlappedComponent :type Primitive%20Component%20Object%20Reference) (OtherActor :type Actor%20Object%20Reference) (OtherComp :type Primitive%20Component%20Object%20Reference) (OtherBodyIndex :type Integer) (bFromSweep :type Boolean) (SweepResult :type Hit%20Result%20Structure%20%28by%20ref%29))
  (if (Actor|ActorHasTag OtherActor "Player")
    (Rendering|Material|SetScalarParameterValue (Variables|Default|GetFogMaterial) "Intensity" 0.3 :!class /Script/Engine.MaterialInstanceDynamic)))

(event OnComponentBeginOverlap(3)
  (params (OverlappedComponent :type Primitive%20Component%20Object%20Reference) (OtherActor :type Actor%20Object%20Reference) (OtherComp :type Primitive%20Component%20Object%20Reference) (OtherBodyIndex :type Integer) (bFromSweep :type Boolean) (SweepResult :type Hit%20Result%20Structure%20%28by%20ref%29))
  (if (Actor|ActorHasTag OtherActor "Player")
    (Rendering|Material|SetScalarParameterValue (Variables|Default|GetFogMaterial) "Intensity" 0.5 :!class /Script/Engine.MaterialInstanceDynamic)))

(event OnComponentBeginOverlap(4)
  (params (OverlappedComponent :type Primitive%20Component%20Object%20Reference) (OtherActor :type Actor%20Object%20Reference) (OtherComp :type Primitive%20Component%20Object%20Reference) (OtherBodyIndex :type Integer) (bFromSweep :type Boolean) (SweepResult :type Hit%20Result%20Structure%20%28by%20ref%29))
  (if (Actor|ActorHasTag OtherActor "Player")
    (Rendering|Material|SetScalarParameterValue (Variables|Default|GetFogMaterial) "Intensity" 0.8 :!class /Script/Engine.MaterialInstanceDynamic)))

(event OnComponentEndOverlap(1)
  (params (OverlappedComponent :type Primitive%20Component%20Object%20Reference) (OtherActor :type Actor%20Object%20Reference) (OtherComp :type Primitive%20Component%20Object%20Reference) (OtherBodyIndex :type Integer))
  (if (Actor|ActorHasTag OtherActor "Player")
    (Rendering|Material|SetScalarParameterValue (Variables|Default|GetFogMaterial) "Intensity" 0.1 :!class /Script/Engine.MaterialInstanceDynamic)))

(event OnComponentEndOverlap(2)
  (params (OverlappedComponent :type Primitive%20Component%20Object%20Reference) (OtherActor :type Actor%20Object%20Reference) (OtherComp :type Primitive%20Component%20Object%20Reference) (OtherBodyIndex :type Integer))
  (if (Actor|ActorHasTag OtherActor "Player")
    (Rendering|Material|SetScalarParameterValue (Variables|Default|GetFogMaterial) "Intensity" 0.2 :!class /Script/Engine.MaterialInstanceDynamic)))

(event OnComponentEndOverlap(3)
  (params (OverlappedComponent :type Primitive%20Component%20Object%20Reference) (OtherActor :type Actor%20Object%20Reference) (OtherComp :type Primitive%20Component%20Object%20Reference) (OtherBodyIndex :type Integer))
  (if (Actor|ActorHasTag OtherActor "Player")
    (Rendering|Material|SetScalarParameterValue (Variables|Default|GetFogMaterial) "Intensity" 0.3 :!class /Script/Engine.MaterialInstanceDynamic)))

(event OnComponentEndOverlap(4)
  (params (OverlappedComponent :type Primitive%20Component%20Object%20Reference) (OtherActor :type Actor%20Object%20Reference) (OtherComp :type Primitive%20Component%20Object%20Reference) (OtherBodyIndex :type Integer))
  (if (Actor|ActorHasTag OtherActor "Player")
    (Rendering|Material|SetScalarParameterValue (Variables|Default|GetFogMaterial) "Intensity" 0.5 :!class /Script/Engine.MaterialInstanceDynamic)))

(event OnComponentBeginOverlap(5)
  (params (OverlappedComponent :type Primitive%20Component%20Object%20Reference) (OtherActor :type Actor%20Object%20Reference) (OtherComp :type Primitive%20Component%20Object%20Reference) (OtherBodyIndex :type Integer) (bFromSweep :type Boolean) (SweepResult :type Hit%20Result%20Structure%20%28by%20ref%29))
  (if (Actor|ActorHasTag OtherActor "Player")
    (Rendering|Material|SetScalarParameterValue (Variables|Default|GetFogMaterial) "Intensity" 1.0 :!class /Script/Engine.MaterialInstanceDynamic)))

(event Custom|UpdateShader
  (Variables|/Script/Engine.PostProcessComponent|SetSettings (Variables|/Game/Tom/Tom_Blueprints/BP_PlayerCharacter.BP_PlayerCharacter_C|GetPostProcess (Variables|Default|GetAs%20BP%20Player%20Character)) (Utilities|Struct|MakePostProcessSettings (Utilities|Struct|MakeWeightedBlendables (Utilities|Array|MakeArray (Utilities|Struct|MakeWeightedBlendable -1.0 (Variables|Default|GetOutlineShaderMaterial)))))))

(event EventBeginPlay
  (bind _returnvalue (Rendering|Material|CreateDynamicMaterialInstance "/Game/Sharan/Materials/M_Fog.M_Fog" "None" "None" :!class /Script/Engine.KismetMaterialLibrary))
  (Variables|Default|SetFogMaterial _returnvalue)
  (Rendering|Material|SetMaterial (Variables|/Game/Sharan/Blueprints/BP_Fog.BP_Fog_C|GetCube (Variables|Default|GetFogBox)) 0 (Variables|Default|GetFogMaterial))
  (bind _asbp_player_character (Utilities|Casting|CastToBP_PlayerCharacter (Game|GetPlayerCharacter 0)))
  (Variables|Default|SetAs%20BP%20Player%20Character _asbp_player_character)
  (bind _returnvalue_2 (Rendering|Material|CreateDynamicMaterialInstance "/Game/James/PP_OutlineShader.PP_OutlineShader" "None" "None" :!class /Script/Engine.KismetMaterialLibrary))
  (Variables|Default|SetOutlineShaderMaterial _returnvalue_2)
  (CallFunction|UpdateShader)
  (Rendering|SetVisibility (Variables|/Game/Sharan/Blueprints/BP_Fog.BP_Fog_C|GetCube (Variables|Default|GetFogBox)) false false))

(event EventTick
  (params (DeltaSeconds :type Float%20%28single-precision%29)))

(fn ConstructionScript)