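; BP_Objectives is an interactable objective pickup for items such as the dress, socks and boots.
; On Interact it identifies the item from Sphere1's static mesh, adds its name to the player's picked-up list, and destroys itself.
; Socks also start the scripted event on BP_BallPoolAndSlide actors, destroying the pickup from inside that loop.
; The player reference comes from the game mode through an interface message at BeginPlay.
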(event Collision|EventActorBeginOverlap
  (params (OtherActor :type Actor%20Object%20Reference))
  (|CallParentFunction OtherActor) ; This node is disabled and will not be called.\nDrag off pins to build functionality.
)

(event EventTick
  (params (DeltaSeconds :type Float%20%28single-precision%29))
  (|CallParentFunction DeltaSeconds) ; This node is disabled and will not be called.\nDrag off pins to build functionality.
)

(event EventInteract
  (params (PlayerRef :type BP%20Player%20Character%20Object%20Reference))
  (bind _sphere1 (Variables|Default|GetSphere1))
  (bind _player_ref (Variables|Default|GetPlayer%20Ref))
  (bind _staticmesh (Variables|/Script/Engine.StaticMeshComponent|GetStaticMesh _sphere1))
  (bind _pickedupitemnames (Variables|/Game/Tom/Tom_Blueprints/BP_PlayerCharacter.BP_PlayerCharacter_C|GetPickedUpItemNames _player_ref))
  (if (== _staticmesh "/Game/Tom/ModelsAndTextures/clothes/Dress_PlaceHolder_/SM_Dress.SM_Dress")
    (Utilities|Array|Add _pickedupitemnames "Dress")
    (Actor|DestroyActor :!label _label)
    (elif (== _staticmesh "/Game/Tom/ModelsAndTextures/clothes/Socks/SM_Socks.SM_Socks")
      (Utilities|Array|Add _pickedupitemnames "Socks")
      (Utilities|FlowControl|DoOnce false
        (:Completed
          (bind _outactors (Actor|GetAllActorsOfClass "/Game/Tom/Tom_Blueprints/BP_BallPoolAndSlide.BP_BallPoolAndSlide_C"))
          (for _array_element _outactors
            (Default|StartScriptedEvent _array_element)
            (goto _label))))
      (elif (== _staticmesh "/Game/Tom/ModelsAndTextures/clothes/Boots/SM_Boots.SM_Boots")
        (Utilities|Array|Add _pickedupitemnames "Boots")
        (goto _label)
        (else
          (goto _label))))))

(event EventBeginPlay
  (bind _gamemoderef (Class|BPIGetGameMode|GetGameModeInterface(Message) (Game|GetGameMode)))
  (Variables|Default|SetGame%20Mode%20Ref _gamemoderef)
  (Variables|Default|SetPlayer%20Ref (Variables|/Game/Tom/Tom_Blueprints/BP_GM_Level1.BP_GM_Level1_C|GetPlayerRef (Variables|Default|GetGame%20Mode%20Ref))))

(fn ConstructionScript
  (|CallParentFunction))

(fn GetObjectiveRef
  (return self))