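; BP_TutorialCoin is a collectible coin for the tutorial level that tells the tutorial player character when it has been collected.
; On BeginPlay it casts player 0's character to BP_Tuorial and caches the reference.
; Its Interact event acts only while the SMCoin component is visible, setting CoinCollect on that character and destroying the coin after a short delay.
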(event EventBeginPlay
  (bind _asbp_tuorial (Utilities|Casting|CastToBP_Tuorial (Game|GetPlayerCharacter 0)))
  (Variables|Default|SetAs%20BP%20Tuorial _asbp_tuorial))

(event EventInteract
  (params (PlayerRef :type BP%20Player%20Character%20Object%20Reference))
  (if (Rendering|IsVisible (Variables|Default|GetSM_Coin))
    (Variables|/Game/Tom/TutorialLevel/BP_Tuorial.BP_Tuorial_C|SetCoinCollect (Variables|Default|GetAs%20BP%20Tuorial) true)
    (Utilities|FlowControl|Delay 0.2)
    (Actor|DestroyActor self)))

(fn ConstructionScript)