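; BP_Tuorial is a first-person-style player pawn, apparently for the tutorial level, with movement, look and interact controls.
; Enhanced Input actions drive movement along the actor's forward and right vectors and feed controller yaw and pitch.
; Interact fires a short visibility line trace from the camera and sends InteractMessage to any hit actor implementing BPI_Interact, keeping interactable logic decoupled from the player.
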(event Input|EnhancedActionEvents|EnhancedInputActionIA_Move
  (params (ActionValue :type Vector%202D%20Structure) (ElapsedSeconds :type Float%20%28double-precision%29) (TriggeredSeconds :type Float%20%28double-precision%29) (InputAction :type Input%20Action%20Object%20Reference :default "/Game/FirstPerson/Input/Actions/IA_Move.IA_Move"))
  ;[1 1 1] Movement mechanics
  (Pawn|Input|AddMovementInput (Transformation|GetActorRightVector) (.x ActionValue) false)
  (Pawn|Input|AddMovementInput (Transformation|GetActorForwardVector) (.y ActionValue) false))

(event Input|EnhancedActionEvents|EnhancedInputActionIA_LookAround
  (params (ActionValue :type Vector%202D%20Structure) (ElapsedSeconds :type Float%20%28double-precision%29) (TriggeredSeconds :type Float%20%28double-precision%29) (InputAction :type Input%20Action%20Object%20Reference :default "/Game/Tom/PlayerInputs/InputActions/IA_LookAround.IA_LookAround"))
  ;[1 1 1] Look Around Mechanics
  (Pawn|Input|AddControllerYawInput (.x ActionValue))
  (Pawn|Input|AddControllerPitchInput (.y ActionValue)))

(event Input|EnhancedActionEvents|EnhancedInputActionIA_Interact
  (params (ActionValue :type Boolean) (ElapsedSeconds :type Float%20%28double-precision%29) (TriggeredSeconds :type Float%20%28double-precision%29) (InputAction :type Input%20Action%20Object%20Reference :default "/Game/Tom/PlayerInputs/InputActions/IA_Interact.IA_Interact"))
  (bind _camera (Variables|Default|GetCamera))
  (bind _returnvalue (Transformation|GetWorldLocation _camera))
  (:Started
    (bind _outhit (Collision|LineTraceByChannel _returnvalue (+ (* (Math|Vector|GetForwardVector _camera) 3e+02) _returnvalue) "TraceTypeQuery1" false 0 "None"))
    (if (Utilities|DoesObjectImplementInterface (.HitActor (Collision|BreakHitResult _outhit)) "/Game/Tom/Tom_Blueprints/BPI_Interact.BPI_Interact_C")
      (Class|BPIInteract|Interact(Message) (.HitActor (Collision|BreakHitResult _outhit))))))

(fn ConstructionScript)