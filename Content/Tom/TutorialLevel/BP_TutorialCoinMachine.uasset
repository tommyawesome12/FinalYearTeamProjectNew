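; Tutorial coin machine that plays a scripted sanity-gain sequence when the player interacts with it while holding a collected coin.
; Sphere overlap enables interaction and shows either an interact prompt or a looping collect-coin prompt, based on the tutorial character's flags.
; Interacting fades in a blinking sanity bar, fills it in delayed steps, then clears SanityGain.
; Tick eases the handle back over a cooldown, which does not block reuse.
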(event OnComponentBeginOverlap(Sphere)
  (params (OverlappedComponent :type Primitive%20Component%20Object%20Reference) (OtherActor :type Actor%20Object%20Reference) (OtherComp :type Primitive%20Component%20Object%20Reference) (OtherBodyIndex :type Integer) (bFromSweep :type Boolean) (SweepResult :type Hit%20Result%20Structure%20%28by%20ref%29))
  (bind _ui (Variables|Default|GetUI))
  (bind _coinui (Variables|Default|GetCoinUI))
  (if (Actor|ActorHasTag OtherActor "Player")
    (Variables|Default|SetCanInteract true)
    (if (Variables|/Game/Tom/TutorialLevel/BP_Tuorial.BP_Tuorial_C|GetCoinCollect (Variables|Default|GetAs%20BP%20Tuorial))
      (UserInterface|Viewport|AddtoViewport (Variables|Default|GetUI) 0)
      (if (Variables|/Game/Tom/TutorialLevel/BP_Tuorial.BP_Tuorial_C|GetSanityGain (Variables|Default|GetAs%20BP%20Tuorial))
        (Utilities|IsValid _ui
          (:Is%20Valid
            (Widget|RemovefromParent _ui))))
      (else
        (UserInterface|Viewport|AddtoViewport _coinui 0)
        (UserInterface|Animation|PlayAnimation _coinui (Variables|/Game/Sharan/CutScenes/CutSceneUI/Interact_UI.Interact_UI_C|GetCollectCoin _coinui) 0.0 100 "Forward" 1.0 false)))))

(event OnComponentEndOverlap(Sphere)
  (params (OverlappedComponent :type Primitive%20Component%20Object%20Reference) (OtherActor :type Actor%20Object%20Reference) (OtherComp :type Primitive%20Component%20Object%20Reference) (OtherBodyIndex :type Integer))
  (bind _ui (Variables|Default|GetUI))
  (bind _coinui (Variables|Default|GetCoinUI))
  (if (Actor|ActorHasTag OtherActor "Player")
    (Variables|Default|SetCanInteract false)
    (if (Variables|/Game/Tom/TutorialLevel/BP_Tuorial.BP_Tuorial_C|GetCoinCollect (Variables|Default|GetAs%20BP%20Tuorial))
      (Utilities|IsValid _ui
        (:Is%20Valid
          (Widget|RemovefromParent _ui)))
      (else
        (Utilities|IsValid _coinui
          (:Is%20Valid
            (Widget|RemovefromParent _coinui)))))))

(event EventBeginPlay
  (bind _asbp_tuorial (Utilities|Casting|CastToBP_Tuorial (Game|GetPlayerCharacter 0)))
  (Variables|Default|SetAs%20BP%20Tuorial _asbp_tuorial)
  (bind _returnvalue (UserInterface|CreateWidget "/Game/Sharan/CutScenes/CutSceneUI/Interact_UI.Interact_UI_C"))
  (Variables|Default|SetUI _returnvalue)
  (bind _returnvalue_2 (UserInterface|CreateWidget "/Game/Sharan/CutScenes/CutSceneUI/Interact_UI.Interact_UI_C"))
  (Variables|Default|SetCoinUI _returnvalue_2))

(event EventTick
  (params (DeltaSeconds :type Float%20%28single-precision%29))
  (bind _cube (Variables|Default|GetCube))
  (bind _ui (Variables|Default|GetUI))
  (bind _coinui (Variables|Default|GetCoinUI))
  (Utilities|FlowControl|Sequence
    (:then_0
      (if (> (Variables|Default|GetNumberOfTimesUsed) 2)
        (Development|SetHiddeninGame (Variables|Default|GetCube1) true false)))
    (:then_1
      (if (Variables|Default|GetUsedMachine)
        (Variables|Default|SetCooldownTimer (+ (Variables|Default|GetCooldownTimer) DeltaSeconds))
        (if (>= (Variables|Default|GetCooldownTimer) 15.0)
          (Variables|Default|SetUsedMachine false)
          (Variables|Default|SetCooldownTimer 0.0))))
    (:then_2
      (if (Variables|Default|GetUsedMachine)
        (Transformation|SetRelativeRotation _cube (Math|Rotator|MakeRotator 0.0 (Math|Float|Lerp -9e+01 0.0 (/ (Variables|Default|GetCooldownTimer) 15.0)) 0.0) false false)
        (else
          (Transformation|SetRelativeRotation _cube (Math|Rotator|MakeRotator 0.0 0.0 0.0) false false))))
    (:then_3
      (if (Variables|/Game/Tom/TutorialLevel/BP_Tuorial.BP_Tuorial_C|GetSanityGain (Variables|Default|GetAs%20BP%20Tuorial))
        (Utilities|IsValid _ui
          (:Is%20Valid
            (Widget|RemovefromParent _ui))
          (:Is%20Not%20Valid
            _))
        (Utilities|IsValid _coinui
          (:Is%20Valid
            (Widget|RemovefromParent _coinui)))))))

(event EventInteract
  (params (PlayerRef :type BP%20Player%20Character%20Object%20Reference))
  (bind _coinui (Variables|Default|GetCoinUI))
  (bind _ui (Variables|Default|GetUI))
  (if (Variables|Default|GetCanInteract)
    (Audio|PlaySound2D "/Game/Sharan/Audio/AudioHorror/MachineHandleBlocked.MachineHandleBlocked" 1.0 1.0 0.0 0 0)
    (if (Variables|/Game/Tom/TutorialLevel/BP_Tuorial.BP_Tuorial_C|GetCoinCollect (Variables|Default|GetAs%20BP%20Tuorial))
      (Utilities|IsValid _coinui
        (:Is%20Valid
          (Widget|RemovefromParent _coinui))
        (:Is%20Not%20Valid
          _))
      (Utilities|IsValid _ui
        (:Is%20Valid
          (Widget|RemovefromParent _ui))
        (:Is%20Not%20Valid
          _))
      (Variables|Default|SetUsedMachine true)
      (Variables|Default|SetCooldownTimer 0.0)
      (bind _returnvalue (UserInterface|CreateWidget "/Game/Sharan/CutScenes/CutSceneUI/SanityGain_UI.SanityGain_UI_C"))
      (bind _output_get (Variables|Default|SetSanityWidget _returnvalue))
      (UserInterface|Viewport|AddtoViewport _output_get 0)
      (UserInterface|Animation|PlayAnimation (Variables|Default|GetSanityWidget) (Variables|/Game/Sharan/CutScenes/CutSceneUI/SanityGain_UI.SanityGain_UI_C|GetFadeIn (Variables|Default|GetSanityWidget)) 0.0 1 "Forward" 1.0 false)
      (UserInterface|Animation|PlayAnimation (Variables|Default|GetSanityWidget) (Variables|/Game/Sharan/CutScenes/CutSceneUI/SanityGain_UI.SanityGain_UI_C|GetBlink (Variables|Default|GetSanityWidget)) 0.0 4 "Forward" 1.0 false)
      (Utilities|FlowControl|Delay 0.5)
      (Progress|SetPercent (Variables|/Game/Sharan/CutScenes/CutSceneUI/SanityGain_UI.SanityGain_UI_C|GetProgressBar_0 (Variables|Default|GetSanityWidget)) 0.65)
      (Utilities|FlowControl|Delay 0.5)
      (Progress|SetPercent (Variables|/Game/Sharan/CutScenes/CutSceneUI/SanityGain_UI.SanityGain_UI_C|GetProgressBar_0 (Variables|Default|GetSanityWidget)) 0.8)
      (Utilities|FlowControl|Delay 0.5)
      (Progress|SetPercent (Variables|/Game/Sharan/CutScenes/CutSceneUI/SanityGain_UI.SanityGain_UI_C|GetProgressBar_0 (Variables|Default|GetSanityWidget)) 1.0)
      (Variables|/Game/Tom/TutorialLevel/BP_Tuorial.BP_Tuorial_C|SetSanityGain (Variables|Default|GetAs%20BP%20Tuorial) false))))

(fn ConstructionScript)