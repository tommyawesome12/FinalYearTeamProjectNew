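; BP_CoinTutorial is an interactable coin pickup for the tutorial level, built on a parent Blueprint.
; Its construction script sets the mesh variable to the coin mesh after running the parent's.
; On BeginPlay it caches the player character as BP_Tuorial.
; On Interact, if its Sphere component is visible, it sets the player's CoinCollect flag and destroys itself.
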(event EventBeginPlay
  (|CallParentFunction)
  (bind _asbp_tuorial (Utilities|Casting|CastToBP_Tuorial (Game|GetPlayerCharacter 0)))
  (Variables|Default|SetAs%20BP%20Tuorial _asbp_tuorial))

(event Collision|EventActorBeginOverlap
  (params (OtherActor :type Actor%20Object%20Reference))
  (|CallParentFunction OtherActor) ; This node is disabled and will not be called.\nDrag off pins to build functionality.
)

(event EventTick
  (params (DeltaSeconds :type Float%20%28single-precision%29))
  (|CallParentFunction DeltaSeconds) ; This node is disabled and will not be called.\nDrag off pins to build functionality.
)

(event EventInteract
  (params (PlayerRef :type BP%20Player%20Character%20Object%20Reference))
  (if (Rendering|IsVisible (Variables|Default|GetSphere))
    (Variables|/Game/Tom/TutorialLevel/BP_Tuorial.BP_Tuorial_C|SetCoinCollect (Variables|Default|GetAs%20BP%20Tuorial) true)
    (Actor|DestroyActor)))

(fn ConstructionScript
  (|CallParentFunction)
  (Variables|Default|SetMeshToUse "/Game/Tom/ModelsAndTextures/Coin/SM_Coin.SM_Coin"))