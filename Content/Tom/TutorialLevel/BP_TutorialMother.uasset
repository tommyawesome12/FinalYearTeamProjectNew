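; BP_TutorialMother is the mother in the tutorial level, advancing tutorial sequences through flags on the player's BP_Tuorial.
; Sphere tracks player proximity and shows the MomInteract_UI prompt once the toy is collected and sequence 2 is unset.
; Interacting nearby with the toy sets PlaySequence2 and destroys Sphere.
; A second trigger, Sphere1, sets PlaySequence4 when the player enters while RunToMom is set.
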(event OnComponentBeginOverlap(Sphere1)
  (params (OverlappedComponent :type Primitive%20Component%20Object%20Reference) (OtherActor :type Actor%20Object%20Reference) (OtherComp :type Primitive%20Component%20Object%20Reference) (OtherBodyIndex :type Integer) (bFromSweep :type Boolean) (SweepResult :type Hit%20Result%20Structure%20%28by%20ref%29))
  (bind _as_bp_tuorial (Variables|Default|GetAs%20BP%20Tuorial))
  (if (Actor|ActorHasTag OtherActor "Player")
    (if (Variables|/Game/Tom/TutorialLevel/BP_Tuorial.BP_Tuorial_C|GetRunToMom _as_bp_tuorial)
      (Variables|/Game/Tom/TutorialLevel/BP_Tuorial.BP_Tuorial_C|SetPlaySequence4 _as_bp_tuorial true))))

(event OnComponentBeginOverlap(Sphere)
  (params (OverlappedComponent :type Primitive%20Component%20Object%20Reference) (OtherActor :type Actor%20Object%20Reference) (OtherComp :type Primitive%20Component%20Object%20Reference) (OtherBodyIndex :type Integer) (bFromSweep :type Boolean) (SweepResult :type Hit%20Result%20Structure%20%28by%20ref%29))
  (bind _as_bp_tuorial (Variables|Default|GetAs%20BP%20Tuorial))
  (if (Actor|ActorHasTag OtherActor "Player")
    (Variables|Default|SetMotherNearby true)
    (if (and (Variables|/Game/Tom/TutorialLevel/BP_Tuorial.BP_Tuorial_C|GetToyCollected? _as_bp_tuorial) (not (Variables|/Game/Tom/TutorialLevel/BP_Tuorial.BP_Tuorial_C|GetPlaySequence2 _as_bp_tuorial)))
      (UserInterface|Viewport|AddtoViewport (Variables|Default|GetMomUI) 0))))

(event OnComponentEndOverlap(Sphere)
  (params (OverlappedComponent :type Primitive%20Component%20Object%20Reference) (OtherActor :type Actor%20Object%20Reference) (OtherComp :type Primitive%20Component%20Object%20Reference) (OtherBodyIndex :type Integer))
  (bind _momui (Variables|Default|GetMomUI))
  (if (Actor|ActorHasTag OtherActor "Player")
    (Variables|Default|SetMotherNearby false)
    (Utilities|IsValid _momui
      (:Is%20Valid
        (Widget|RemovefromParent _momui)))))

(event EventBeginPlay
  (bind _asbp_tuorial (Utilities|Casting|CastToBP_Tuorial (Game|GetPlayerCharacter 0)))
  (Variables|Default|SetAs%20BP%20Tuorial _asbp_tuorial)
  (bind _returnvalue (UserInterface|CreateWidget "/Game/Sharan/CutScenes/CutSceneUI/MomInteract_UI.MomInteract_UI_C"))
  (Variables|Default|SetMomUI _returnvalue))

(event EventInteract
  (params (PlayerRef :type BP%20Player%20Character%20Object%20Reference))
  (if (and (Variables|Default|GetMotherNearby) (Variables|/Game/Tom/TutorialLevel/BP_Tuorial.BP_Tuorial_C|GetToyCollected? (Variables|Default|GetAs%20BP%20Tuorial)))
    (Variables|/Game/Tom/TutorialLevel/BP_Tuorial.BP_Tuorial_C|SetPlaySequence2 (Variables|Default|GetAs%20BP%20Tuorial) true)
    (Components|DestroyComponent (Variables|Default|GetSphere))))

(fn ConstructionScript)