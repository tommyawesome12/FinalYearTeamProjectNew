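; BP_Wizard is a tutorial-level wizard actor that the player interacts with once to take the Starmy in its hand.
; An overlap sphere enables collection for Player-tagged actors and shows a pulsing prompt widget created at BeginPlay.
; The first valid Interact hides the held Starmy, swaps the prompt for a second widget that fades in and out over timed delays, then destroys the actor.
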(event OnComponentBeginOverlap(Sphere)
  (params (OverlappedComponent :type Primitive%20Component%20Object%20Reference) (OtherActor :type Actor%20Object%20Reference) (OtherComp :type Primitive%20Component%20Object%20Reference) (OtherBodyIndex :type Integer) (bFromSweep :type Boolean) (SweepResult :type Hit%20Result%20Structure%20%28by%20ref%29))
  (if (Actor|ActorHasTag OtherActor "Player")
    (Variables|Default|SetCanCollect true)
    (UserInterface|Viewport|AddtoViewport (stale EventBeginPlay _output_get) 0)
    (UserInterface|Animation|PlayAnimation (stale EventBeginPlay _output_get) (Variables|/Game/Sharan/CutScenes/CutSceneUI/Interact_UI.Interact_UI_C|GetFade (stale EventBeginPlay _output_get)) 0.0 10000 "Forward" 0.7 false)))

(event OnComponentEndOverlap(Sphere)
  (params (OverlappedComponent :type Primitive%20Component%20Object%20Reference) (OtherActor :type Actor%20Object%20Reference) (OtherComp :type Primitive%20Component%20Object%20Reference) (OtherBodyIndex :type Integer))
  (if (Actor|ActorHasTag OtherActor "Player")
    (Variables|Default|SetCanCollect false)
    (Utilities|IsValid (stale EventBeginPlay _returnvalue)
      (:Is%20Valid
        (Widget|RemovefromParent (stale EventBeginPlay _output_get))))))

(event EventInteract
  (params (PlayerRef :type BP%20Player%20Character%20Object%20Reference))
  (bind _ui (Variables|Default|GetUI))
  (Development|PrintString "Hello")
  (if (Variables|Default|GetCanCollect)
    (Utilities|FlowControl|DoOnce false
      (:Completed
        (Rendering|SetVisibility (Variables|Default|GetStarmyInHand__1_) false false)
        (Utilities|IsValid _ui
          (:Is%20Valid
            (Widget|RemovefromParent _ui)
            (Utilities|FlowControl|Delay 0.1)
            (bind _returnvalue (UserInterface|CreateWidget "/Game/Sharan/CutScenes/CutSceneUI/Interact2_UI.Interact2_UI_C"))
            (UserInterface|Viewport|AddtoViewport _returnvalue 0)
            (UserInterface|Animation|PlayAnimation _returnvalue (Variables|/Game/Sharan/CutScenes/CutSceneUI/Interact2_UI.Interact2_UI_C|GetFade _returnvalue) 0.0 1 "Forward" 1.0 false)
            (Utilities|FlowControl|Delay 4.0)
            (UserInterface|Animation|PlayAnimation _returnvalue (Variables|/Game/Sharan/CutScenes/CutSceneUI/Interact2_UI.Interact2_UI_C|GetFade _returnvalue) 0.0 1 "Reverse" 1.0 false)
            (Utilities|FlowControl|Delay 2.5)
            (Actor|DestroyActor)))))))

(event EventBeginPlay
  (bind _returnvalue (UserInterface|CreateWidget "/Game/Sharan/CutScenes/CutSceneUI/Interact_UI.Interact_UI_C"))
  (bind _output_get (Variables|Default|SetUI _returnvalue)))

(fn ConstructionScript)