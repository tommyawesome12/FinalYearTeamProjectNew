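; Level 1 game mode for a sanity-based horror game with mannequins, collectible clothing objectives and coins.
; BeginPlay caches level actors, then spawns objectives and coins at random spawn points, destroying each used point.
; While InBadPlace, sanity drains, and UpdateSanity fans changes out to props, clothes and lights, triggering warnings, a scream and flickering.
; Callable scare events temporarily increase drain, while the random event timer currently only plays sounds near the player.
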(event Custom|Record%20Pickup
  (params (Collected :type Integer))
  (bind _output_get (Variables|Default|SetCollectedItems Collected))
  (Default|ItemCollected (Variables|Default|GetMotherRef) _output_get))

(event Custom|UpdateSanity
  (params (SanityValue :type Float%20%28double-precision%29))
  (Utilities|FlowControl|Sequence
    (:then_0
      (for _array_element (Variables|Default|GetPlacedObjectsArray)
        (Default|UpdateTexture _array_element SanityValue)))
    (:then_1
      (for _array_element_2 (Variables|Default|GetClothesRackArray)
        (Default|UpdateClothes _array_element_2 SanityValue)))
    (:then_2
      (if (<= SanityValue 0.1)
        (Variables|Default|SetLightsFlicker true)
        (else
          (Variables|Default|SetLightsFlicker false))))
    (:then_3
      (if (<= SanityValue 0.3)
        (Utilities|FlowControl|DoOnce false
          (:Completed
            (Camera|PlayWorldCameraShake "/Game/Tom/Tom_Blueprints/BP_CameraShake.BP_CameraShake_C" (Transformation|GetActorLocation (Variables|Default|GetPlayerRef)) 0.0 3e+02)
            (Audio|PlaySound2D "/Game/Sharan/Audio/SoundCues/Scream_Cue.Scream_Cue" 1.0 1.0 0.0 0 0)
            (Variables|Default|SetCanTick false)))))
    (:then_4
      (for _array_element_3 (Variables|Default|GetLightsVariable)
        (Default|UpdateLighting _array_element_3 SanityValue)))
    (:then_5
      (if (<= SanityValue 0.35)
        (Utilities|FlowControl|DoOnce false
          (:Completed
            (Audio|PlaySound2D "/Game/Sharan/Audio/SoundsForTom/SanityWarning.SanityWarning" 1.0 1.0 0.0 0 0)
            (CallFunction|SanityWarning)))))))

(event Custom|StopMannequinMoving
  (for _array_element (Variables|Default|GetArrayOfMannequinnes)
    (Default|StopLogic _array_element)))

(event Custom|SanityDrainOverTime
  (params (DrainAmount :type Float%20%28double-precision%29))
  (if (Variables|Default|GetInBadPlace)
    (Default|DecreaseSanity (Variables|Default|GetPlayerRef) DrainAmount)))

(event Custom|LightFlickering
  (params (TimeDelta :type Float%20%28double-precision%29))
  (bind _blinkingwidget (Variables|Default|GetBlinkingWidget))
  (bind _blinkingwidget_2 (Variables|Default|GetBlinkingWidget))
  ;[1 1 1] light flickering mechanic for when sanity is low enough
  (if (Variables|Default|GetLightsFlicker)
    (Widget|SetVisibility (Variables|Default|GetBlinkingWidget) "Visible")
    (if (Variables|Default|GetLightsOn)
      (bind _output_get (Variables|Default|SetLightsTimer (+ (Variables|Default|GetLightsTimer) TimeDelta)))
      (if (>= _output_get (Math|Random|RandomFloatinRange 2.0 5.0))
        (Variables|Default|SetLightsOn false)
        (Variables|Default|SetLightsTimer 0.0)
        (for _array_element (Variables|Default|GetLightsVariable)
          (Default|TurnLightOff _array_element)
          (UserInterface|Animation|PlayAnimation _blinkingwidget_2 (Variables|/Game/Sharan/UI/BP_BlinkingEffect.BP_BlinkingEffect_C|GetFade _blinkingwidget_2) 0.0 1 "Forward" 1.0 false))
        (for _array_element_2 (Variables|Default|GetArrayOfMannequinnes)
          (Variables|/Game/Sharan/Blueprints/RBP_Mannequine1.RBP_Mannequine1_C|SetLightsOn _array_element_2 false)))
      (else
        (bind _output_get_2 (Variables|Default|SetLightsTimer (+ (Variables|Default|GetLightsTimer) TimeDelta)))
        (if (>= _output_get_2 1.0)
          (Variables|Default|SetLightsOn true)
          (Variables|Default|SetLightsTimer 0.0)
          (for _array_element_3 (Variables|Default|GetLightsVariable)
            (Default|TurnLighton _array_element_3)
            (UserInterface|Animation|PlayAnimation _blinkingwidget (Variables|/Game/Sharan/UI/BP_BlinkingEffect.BP_BlinkingEffect_C|GetFade _blinkingwidget) 0.0 1 "Reverse" 1.0 false))
          (for _array_element_4 (Variables|Default|GetArrayOfMannequinnes)
            (Variables|/Game/Sharan/Blueprints/RBP_Mannequine1.RBP_Mannequine1_C|SetLightsOn _array_element_4 true)))))))

(event Custom|StartMannequinMoving
  (for _array_element (Variables|Default|GetArrayOfMannequinnes)
    (Default|StartLogic _array_element)))

(event Custom|UpdateMannequinneLoction
  (for _array_element (Variables|Default|GetArrayOfMannequinnes)
    (Default|TeleporttoStartPosition _array_element)))

(event Custom|SanityWarning
  (if (Variables|Default|GetCanTick)
    (Audio|PlaySound2D "/Game/Sharan/Audio/SoundsForTom/SanityTicking.SanityTicking" 1.0 1.0 0.0 0 0)
    (Utilities|FlowControl|Delay 2.5)
    (CallFunction|SanityWarning)))

(event EventBeginPlay
  (bind _returnvalue (UserInterface|CreateWidget "/Game/Sharan/UI/BP_BlinkingEffect.BP_BlinkingEffect_C"))
  (bind _output_get (Variables|Default|SetBlinkingWidget _returnvalue))
  (UserInterface|Viewport|AddtoViewport _output_get 0)
  (Widget|SetVisibility (Variables|Default|GetBlinkingWidget) "Hidden")
  (bind _outactors (Actor|GetAllActorsOfClass "/Game/Sharan/Blueprints/BP_Objectives.BP_Objectives_C"))
  (Variables|Default|SetTotalItems (Utilities|Array|Length _outactors))
  (bind _returnvalue_2 (Actor|GetActorOfClass "/Game/Tom/Tom_Blueprints/BP_Mother.BP_Mother_C"))
  (Variables|Default|SetMotherRef _returnvalue_2)
  (bind _outactors_2 (Actor|GetAllActorsOfClass "/Game/Tom/Tom_Blueprints/BP_PlacedObjects.BP_PlacedObjects_C"))
  (Variables|Default|SetPlacedObjectsArray _outactors_2)
  (bind _outactors_3 (Actor|GetAllActorsOfClass "/Game/Tom/Tom_Blueprints/BP_Lights.BP_Lights_C"))
  (Variables|Default|SetLightsVariable _outactors_3)
  (bind _outactors_4 (Actor|GetAllActorsOfClass "/Game/Tom/Tom_Blueprints/BP_CothesRandomiser.BP_CothesRandomiser_C"))
  (Variables|Default|SetClothesRackArray _outactors_4)
  (bind _outactors_5 (Actor|GetAllActorsOfClass "/Game/Tom/Tom_Blueprints/BP_HangerObjectiveSpawn.BP_HangerObjectiveSpawn_C"))
  (Variables|Default|SetHangerSpawnPoints _outactors_5)
  (bind _outactors_6 (Actor|GetAllActorsOfClass "/Game/Tom/Tom_Blueprints/BP_PigeonHoleObjectiveSpawn.BP_PigeonHoleObjectiveSpawn_C"))
  (Variables|Default|SetPigeonHoleSpawnPoints _outactors_6)
  (bind _returnvalue_3 (Actor|GetActorOfClass "/Game/Tom/Tom_Blueprints/BP_PlayerCharacter.BP_PlayerCharacter_C"))
  (Variables|Default|SetPlayerRef _returnvalue_3)
  (bind _outactors_7 (Actor|GetAllActorsOfClass "/Game/Sharan/Blueprints/RBP_Mannequine1.RBP_Mannequine1_C"))
  (Variables|Default|SetArrayOfMannequinnes _outactors_7)
  (CallFunction|SpawnObjectives)
  (CallFunction|EventGraphBeginPlay)
  (CallFunction|SpawnCoins))

(event EventTick
  (params (DeltaSeconds :type Float%20%28single-precision%29))
  (CallFunction|SanityDrainOverTime (/ DeltaSeconds (Variables|Default|GetDuration)))
  (CallFunction|EventGraphonTick DeltaSeconds)
  (if (Variables|/Game/Tom/Tom_Blueprints/BP_PlayerCharacter.BP_PlayerCharacter_C|GetCanFadeToBlack (Variables|Default|GetPlayerRef))
    (if (Variables|Default|GetInBadPlace)
      (CallFunction|LightFlickering DeltaSeconds))))

(event Custom|EventGraphBeginPlay
  ;[1 1 1] EventCalling
)

(event Custom|EventGraphOnTick
  (params (DeltaTime :type Float%20%28double-precision%29))
  ;[1 1 1] EventCalling
  (if (Variables|Default|GetInBadPlace)
    (Utilities|FlowControl|Sequence
      (:then_0
        (Variables|Default|SetEventCooldown (+ DeltaTime (Variables|Default|GetEventCooldown)))
        (Variables|Default|SetTimerForEvents (+ DeltaTime (Variables|Default|GetTimerForEvents)))
        (if (>= (Variables|Default|GetTimerForEvents) (Math|Random|RandomFloatinRange 15.0 2e+01))
          (if (>= (Variables|Default|GetEventCooldown) 0.0)
            (Variables|Default|SetTimerForEvents 0.0)
            (Variables|Default|SetEventCooldown 0.0)
            (CallFunction|SelectRandomEvent))))
      (:then_1
        (if (Variables|Default|GetEventHappening)
          (Default|DecreaseSanity (Variables|Default|GetPlayerRef) (/ DeltaTime (Variables|Default|GetEventDecreaseAmount)))))
      (:then_2
        (if (Variables|Default|GetEventHappening)
          (bind _outactors (Actor|GetAllActorsOfClass "/Game/Tom/Tom_Blueprints/BP_FakeMannequin.BP_FakeMannequin_C"))
          (Utilities|IsValid (Utilities|Array|Get(acopy) _outactors)
            (:Is%20Not%20Valid
              (Variables|Default|SetEventHappening false))))))))

(event Custom|Random%20Audio
  (bind _soundarray (Variables|Default|GetSoundArray))
  ;[1 1 1] TensionBuildup Events
  (bind _randomlocation (Class|NavigationSystemV1|GetRandomLocationinNavigableRadius (Transformation|GetActorLocation (Variables|Default|GetPlayerRef)) 2e+02 0 0))
  (Audio|PlaySoundatLocation (Utilities|Array|Get(acopy) _soundarray (Math|Random|RandomIntegerinRange 0 (- (Utilities|Array|Length _soundarray) 1))) _randomlocation "0, 0, 0" 1.0 1.0 0.0 0 0 0 0))

(event Custom|ServiceAnnouncement
  ;[1 1 1] Tension Release Events
)

(event Custom|HeadJumpAtYou
  (params (HeadRef :type BP%20Jumping%20Head%20Object%20Reference))
  ;[1 1 1] Tension Release Events
  (Utilities|IsValid HeadRef
    (:Is%20Valid
      (Default|JumpatPlayer HeadRef)
      (Variables|Default|SetEventHappening true)
      (Variables|Default|SetEventDecreaseAmount 5e+01)
      (Utilities|FlowControl|Delay 0.5)
      (Variables|Default|SetEventHappening false))))

(event Custom|ShelfFallingOver
  (params (RackRef :type BP%20Falling%20Rack%20Object%20Reference))
  ;[1 1 1] Tension Release Events
  (Default|Fallen RackRef)
  (Variables|Default|SetEventHappening true)
  (Variables|Default|SetEventDecreaseAmount 5e+01)
  (Utilities|FlowControl|Delay 0.5)
  (Variables|Default|SetEventHappening false))

(event Custom|FinishSingleRedLightEvent
  ;[1 1 1] TensionBuildup Events
  (Widget|RemovefromParent (Variables|Default|GetCameraFilterRef))
  (bind _outactors (Actor|GetAllActorsOfClass "/Game/Tom/Tom_Blueprints/BP_Lights.BP_Lights_C"))
  (for _array_element _outactors
    (Default|TurnLighton _array_element))
  (Variables|Default|SetEventHappening false))

(event Custom|CallCameraFallEvent
  (params (Camera :type BP%20Follow%20Camera%20Object%20Reference))
  ;[1 1 1] TensionBuildup Events
  (Variables|Default|SetTimerForEvents 0.0)
  (Utilities|IsValid Camera
    (:Is%20Valid
      (Default|Fall Camera)
      (Variables|Default|SetEventHappening true)
      (Variables|Default|SetEventDecreaseAmount 5e+01)
      (Utilities|FlowControl|Delay 0.3)
      (Variables|Default|SetEventHappening false))))

(event Custom|CallBallRollEvent
  ;[1 1 1] TensionBuildup Events
)

(event Custom|CallSingleRedLightEvent
  (params (Light :type BP%20Lights%20Object%20Reference))
  ;[1 1 1] TensionBuildup Events
  (Variables|Default|SetTimerForEvents 0.0)
  (Default|TurnLightRed Light)
  (bind _outactors (Actor|GetAllActorsOfClass "/Game/Tom/Tom_Blueprints/BP_Lights.BP_Lights_C"))
  (bind _output_get (Variables|Default|SetLightsToTurnOff _outactors))
  (Utilities|Array|RemoveItem _output_get Light)
  (for _array_element (Variables|Default|GetLightsToTurnOff)
    (Default|TurnLightOff _array_element))
  (bind _returnvalue (UserInterface|CreateWidget "/Game/Sharan/UI/WIG_CameraFilter.WIG_CameraFilter_C" (Game|GetPlayerController 0)))
  (Variables|Default|SetCameraFilterRef _returnvalue)
  (UserInterface|Viewport|AddtoViewport _returnvalue 0)
  (Default|GetReferences _returnvalue self Light)
  (Variables|Default|SetEventDecreaseAmount 1e+02)
  (Variables|Default|SetEventHappening true))

(event Custom|CallShakeRacksEvent
  (params (Racks :type Array%20of%20BP%20Movable%20Racks%20Object%20References))
  ;[1 1 1] TensionBuildup Events
  (for _array_element Racks
    (Default|Shake _array_element)
    (Variables|Default|SetEventHappening true)
    (Variables|Default|SetEventDecreaseAmount 1e+02)
    (Utilities|FlowControl|Delay 1.2)
    (Variables|Default|SetEventHappening false)))

(event Custom|CallCrunchSoundEvent
  ;[1 1 1] TensionBuildup Events
)

(event Custom|CallLightFallEvent
  (params (Light :type BP%20Lights%20Object%20Reference))
  ;[1 1 1] TensionBuildup Events
  (Variables|Default|SetTimerForEvents 0.0)
  (Default|Fall Light)
  (Variables|Default|SetEventHappening true)
  (Variables|Default|SetEventDecreaseAmount 5e+01)
  (Utilities|FlowControl|Delay 0.3)
  (Variables|Default|SetEventHappening false))

(event Custom|CallClothesFallEvent
  (params (Cloths :type BP%20Cothes%20Randomiser%20Object%20Reference))
  ;[1 1 1] TensionBuildup Events
)

(event Custom|Spawn%20Coins
  ;[1 1 1] SpawnsCoins
  (if (not (>= (Variables|Default|GetCoinCount) 11))
    (bind _outactors (Actor|GetAllActorsOfClass "/Game/Tom/Tom_Blueprints/BP_CoinsSpawn.BP_CoinsSpawn_C"))
    (bind _success (CallFunction|RandomSpawnObject _outactors "/Game/Tom/Tom_Blueprints/BP_CoinPickup.BP_CoinPickup_C" "1.000000,1.000000,1.000000"))
    (if _success
      (Math|Integer|IncrementInt (Variables|Default|GetCoinCount)
        (:%20%20
          (CallFunction|SpawnCoins)))
      (else
        (CallFunction|SpawnCoins)))))

(event Custom|Spawn%20Objectives
  ;[1 1 1] SpawnsCoins
  (CallFunction|SpawnDress)
  (CallFunction|SpawnSocks)
  (CallFunction|SpawnBoots))

(event Custom|SpawnSocks
  ;[1 1 1] SpawnsCoins
  (bind _outactors (Actor|GetAllActorsOfClass "/Game/Tom/Tom_Blueprints/BP_SocksSpawn.BP_SocksSpawn_C"))
  (bind (_success _spawnedobjectdetails) (CallFunction|RandomSpawnObject _outactors "/Game/Sharan/Blueprints/BP_Objectives.BP_Objectives_C" "1.000000,1.000000,1.000000"))
  (if _success
    (bind _objectiveref (Class|BPIGetObjectiveRef|GetObjectiveRef(Message) _spawnedobjectdetails))
    (Utilities|IsValid _objectiveref
      (:Is%20Valid
        (Variables|/Game/Tom/Tom_Blueprints/BP_PickupBase.BP_PickupBase_C|SetMeshToUse _objectiveref "/Game/Tom/ModelsAndTextures/clothes/Socks/SM_Socks.SM_Socks")
        (Variables|/Game/Tom/Tom_Blueprints/BP_PickupBase.BP_PickupBase_C|SetMaterialToUse _objectiveref "/Game/Tom/ModelsAndTextures/clothes/Socks/M_Socks.M_Socks")
        (Default|UpdateLooks _objectiveref))
      (:Is%20Not%20Valid
        (CallFunction|SpawnSocks)))
    (else
      (CallFunction|SpawnSocks))))

(event Custom|SpawnDress
  ;[1 1 1] SpawnsCoins
  (bind _outactors (Actor|GetAllActorsOfClass "/Game/Tom/Tom_Blueprints/BP_DressSpawn.BP_DressSpawn_C"))
  (bind (_success _spawnedobjectdetails) (CallFunction|RandomSpawnObject _outactors "/Game/Sharan/Blueprints/BP_Objectives.BP_Objectives_C" "1.000000,1.000000,1.000000"))
  (if _success
    (bind _objectiveref (Class|BPIGetObjectiveRef|GetObjectiveRef(Message) _spawnedobjectdetails))
    (Utilities|IsValid _objectiveref
      (:Is%20Valid
        (Variables|/Game/Tom/Tom_Blueprints/BP_PickupBase.BP_PickupBase_C|SetMeshToUse _objectiveref "/Game/Tom/ModelsAndTextures/clothes/Dress_PlaceHolder_/SM_Dress.SM_Dress")
        (Variables|/Game/Tom/Tom_Blueprints/BP_PickupBase.BP_PickupBase_C|SetMaterialToUse _objectiveref "/Game/Tom/ModelsAndTextures/clothes/Dress_PlaceHolder_/M_Dress.M_Dress")
        (Default|UpdateLooks _objectiveref))
      (:Is%20Not%20Valid
        (CallFunction|SpawnDress)))
    (else
      (CallFunction|SpawnDress))))

(event Custom|SpawnBoots
  ;[1 1 1] SpawnsCoins
  (bind _outactors (Actor|GetAllActorsOfClass "/Game/Tom/Tom_Blueprints/BP_BootsSpawn.BP_BootsSpawn_C"))
  (bind (_success _spawnedobjectdetails) (CallFunction|RandomSpawnObject _outactors "/Game/Sharan/Blueprints/BP_Objectives.BP_Objectives_C" "2.000000,2.000000,2.000000"))
  (if _success
    (bind _objectiveref (Class|BPIGetObjectiveRef|GetObjectiveRef(Message) _spawnedobjectdetails))
    (Utilities|IsValid _objectiveref
      (:Is%20Valid
        (Variables|/Game/Tom/Tom_Blueprints/BP_PickupBase.BP_PickupBase_C|SetMeshToUse _objectiveref "/Game/Tom/ModelsAndTextures/clothes/Boots/SM_Boots.SM_Boots")
        (Variables|/Game/Tom/Tom_Blueprints/BP_PickupBase.BP_PickupBase_C|SetMaterialToUse _objectiveref "/Game/Tom/ModelsAndTextures/clothes/Boots/M_NewBoots.M_NewBoots")
        (Default|UpdateLooks _objectiveref))
      (:Is%20Not%20Valid
        (CallFunction|SpawnBoots)))
    (else
      (CallFunction|SpawnBoots))))

(fn ConstructionScript)

(fn RandomSpawnObject
  (params (ArrayOfSpawnPoints :type Array%20of%20Actor%20Object%20References) (ActorTypeToSpawn :type Actor%20Class%20Reference) (RelativeScale :type Vector))
  (LocalVariables|SetRandomInt (Math|Random|RandomIntegerinRange 0 (- (Utilities|Array|Length ArrayOfSpawnPoints) 1)))
  (Utilities|IsValid (Utilities|Array|Get(acopy) ArrayOfSpawnPoints (LocalVariables|GetRandomInt))
    (:Is%20Valid
      (bind _returnvalue (Game|SpawnActorfromClass ActorTypeToSpawn (Math|Transform|MakeTransform (Transformation|GetActorLocation (Utilities|Array|Get(acopy) ArrayOfSpawnPoints (LocalVariables|GetRandomInt))) "0, 0, 0" RelativeScale) "Undefined" "MultiplyWithRoot" 0 0))
      (Actor|DestroyActor (Utilities|Array|Get(acopy) ArrayOfSpawnPoints (LocalVariables|GetRandomInt)))
      (return true _returnvalue))
    (:Is%20Not%20Valid
      (return false 0))))

(fn SelectRandomEvent
  (Math|Integer|CompareInt (Math|Random|RandomIntegerinRange 0 1) 1
    (:==
      (if (<= (Variables|/Game/Tom/Tom_Blueprints/BP_PlayerCharacter.BP_PlayerCharacter_C|GetSanity (Variables|Default|GetPlayerRef)) 0.45)
        _
        (else
          _))
      (CallFunction|SelectRandomEvent))
    (:<
      (CallFunction|RandomAudio))))

(fn FadeToblack
  (bind _blinkingwidget (Variables|Default|GetBlinkingWidget))
  (Widget|SetVisibility (Variables|Default|GetBlinkingWidget) "Visible")
  (UserInterface|Animation|PlayAnimation _blinkingwidget (Variables|/Game/Sharan/UI/BP_BlinkingEffect.BP_BlinkingEffect_C|GetFade _blinkingwidget) 0.0 1 "Forward" 1.0 false))

(fn FadefromBlack
  (bind _blinkingwidget (Variables|Default|GetBlinkingWidget))
  (UserInterface|Animation|PlayAnimation _blinkingwidget (Variables|/Game/Sharan/UI/BP_BlinkingEffect.BP_BlinkingEffect_C|GetFade _blinkingwidget) 0.0 1 "Reverse" 1.0 false))

(fn GetGameModeInterface
  (return self))

(fn GetObjectiveRef
  (return 0))