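; BP_CoinPickup is a collectible coin that the player picks up through an Interact event.
; Interact increments the Coins count on the passed player reference, plays a collect sound, shows a newly created coin count widget, then destroys the actor.
; The construction script calls the parent and sets MeshToUse to the coin mesh, while overlap handling is disabled.
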(event EventBeginPlay
  (|CallParentFunction))

(event Collision|EventActorBeginOverlap
  (params (OtherActor :type Actor%20Object%20Reference))
  (|CallParentFunction OtherActor) ; This node is disabled and will not be called.\nDrag off pins to build functionality.
)

(event EventTick
  (params (DeltaSeconds :type Float%20%28single-precision%29))
  (|CallParentFunction DeltaSeconds))

(event EventInteract
  (params (PlayerRef :type BP%20Player%20Character%20Object%20Reference))
  (Math|Integer|IncrementInt (Variables|/Game/Tom/Tom_Blueprints/BP_PlayerCharacter.BP_PlayerCharacter_C|GetCoins PlayerRef)
    (:%20%20
      (Audio|PlaySound2D "/Game/Sharan/Audio/AudioHorror/CoinCollect.CoinCollect" 1.0 1.0 0.0 0 0)
      (bind _returnvalue (UserInterface|CreateWidget "/Game/Sharan/UI/BP_WIG_CoinCount.BP_WIG_CoinCount_C"))
      (UserInterface|Viewport|AddtoViewport _returnvalue 0)
      (Actor|DestroyActor))))

(fn ConstructionScript
  (|CallParentFunction)
  (Variables|Default|SetMeshToUse "/Game/Tom/ModelsAndTextures/Coin/SM_Coin.SM_Coin"))