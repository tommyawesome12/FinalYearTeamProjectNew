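; BP_FootPrintSpline is an actor that lays a trail of footprints along a spline.
; On BeginPlay it spawns BP_FootPrint actors at a fixed distance interval along the spline, with the count derived from the spline's length.
; Each footprint is rotated to the spline's tangent and receives the InstanceToUse material instance.
; The construction script holds only an empty loop, so placement happens at runtime.
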(event EventBeginPlay
  (bind _spline (Variables|Default|GetSpline))
  (for _index (range 0 (- (Math|Float|Round (/ (Spline|GetSplineLength _spline) 3e+02)) 1))
    (bind _returnvalue (Game|SpawnActorfromClass "/Game/Tom/Tom_Blueprints/BP_FootPrint.BP_FootPrint_C" (Math|Transform|MakeTransform (Spline|GetLocationatDistanceAlongSpline _spline (* _index 3e+02) "World") (Math|Conversions|RotationFromXVector (Spline|GetTangentatDistanceAlongSpline (Variables|Default|GetSpline) (* _index 3e+02) "World")) "1.000000,1.000000,1.000000") "Undefined" "MultiplyWithRoot" 0 0))
    (Variables|/Game/Tom/Tom_Blueprints/BP_FootPrint.BP_FootPrint_C|SetMaterialInstance _returnvalue (Variables|Default|GetInstanceToUse))))

(event Collision|EventActorBeginOverlap
  (params (OtherActor :type Actor%20Object%20Reference)))

(event EventTick
  (params (DeltaSeconds :type Float%20%28single-precision%29)))

(fn ConstructionScript
  (for _index (range 0 (- 0 1))
    _))