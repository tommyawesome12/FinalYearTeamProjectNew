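; BP_PlacedObjects is a configurable placed mesh actor whose material shifts between "good" and "bad" texture sets according to a Sanity value.
; The construction script assigns the mesh and builds a dynamic material instance, filling it with good and bad base colour, ORM and normal textures.
; BeginPlay sets a starting Sanity parameter, and the UpdateTexture event later drives it from an incoming sanity value, offset and clamped.
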(event Custom|UpdateTexture
  (params (SanityValue :type Float%20%28double-precision%29))
  (if true
    (Rendering|Material|SetScalarParameterValue (Variables|Default|GetDynamicMaterialInstance) "Sanity" (Math|Float|Clamp(Float) (- SanityValue 0.5)) :!class /Script/Engine.MaterialInstanceDynamic)))

(event EventBeginPlay
  (Rendering|Material|SetScalarParameterValue (Variables|Default|GetDynamicMaterialInstance) "Sanity" 0.5 :!class /Script/Engine.MaterialInstanceDynamic))

(event Collision|EventActorBeginOverlap
  (params (OtherActor :type Actor%20Object%20Reference)))

(fn ConstructionScript
  (bind _staticmesh (Variables|Default|GetStaticMesh))
  (Components|StaticMesh|SetStaticMesh _staticmesh (Variables|Default|GetMesh))
  (bind _returnvalue (Rendering|Material|CreateDynamicMaterialInstance (Variables|Default|GetMaterialInstace) "None" "None" :!class /Script/Engine.KismetMaterialLibrary))
  (Variables|Default|SetDynamicMaterialInstance _returnvalue)
  (Rendering|Material|SetTextureParameterValue _returnvalue "GoodTextureBaseColour" (Variables|Default|GetGoodTextureBaseColour))
  (Rendering|Material|SetTextureParameterValue _returnvalue "BadTextureBaseColour" (Variables|Default|GetBadTextureBaseColour))
  (Rendering|Material|SetTextureParameterValue _returnvalue "GoodTextureORM" (Variables|Default|GetGoodTextureORM))
  (Rendering|Material|SetTextureParameterValue _returnvalue "BadTextureORM" (Variables|Default|GetBadTextureORM))
  (Rendering|Material|SetTextureParameterValue _returnvalue "GoodTextureNormal" (Variables|Default|GetGoodTextureNormal))
  (Rendering|Material|SetTextureParameterValue _returnvalue "BadTextureNormal" (Variables|Default|GetBadTextureNormal))
  (Rendering|Material|SetScalarParameterValue _returnvalue "Sanity" 1.0 :!class /Script/Engine.MaterialInstanceDynamic)
  (Rendering|Material|SetMaterial _staticmesh 0 _returnvalue))