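; BP_CoinMachine is an interactable machine that trades one of the player's coins for a small Sanity increase, up to three uses.
; Interact requires remaining uses, a coin and Sanity below a near-full threshold, then deducts the coin, calls IncreaseSanity and adds a new BP_WIG_CoinCount widget to the viewport.
; Tick polls the use count and hides Cube1 once the machine is used up.
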(event EventBeginPlay)

(event Collision|EventActorBeginOverlap
  (params (OtherActor :type Actor%20Object%20Reference)))

(event EventTick
  (params (DeltaSeconds :type Float%20%28single-precision%29))
  (if (> (Variables|Default|GetNumberOfTimesUsed) 2)
    (Development|SetHiddeninGame (Variables|Default|GetCube1) true false)))

(event EventInteract
  (params (PlayerRef :type BP%20Player%20Character%20Object%20Reference))
  (bind _coins (Variables|/Game/Tom/Tom_Blueprints/BP_PlayerCharacter.BP_PlayerCharacter_C|GetCoins PlayerRef))
  (bind _numberoftimesused (Variables|Default|GetNumberOfTimesUsed))
  (if (< _numberoftimesused 3)
    (if (> _coins 0)
      (if (< (Variables|/Game/Tom/Tom_Blueprints/BP_PlayerCharacter.BP_PlayerCharacter_C|GetSanity PlayerRef) 0.95)
        (Math|Integer|DecrementInt _coins
          (:%20%20
            (Math|Integer|IncrementInt _numberoftimesused
              (:%20%20
                (bind _returnvalue (UserInterface|CreateWidget "/Game/Sharan/UI/BP_WIG_CoinCount.BP_WIG_CoinCount_C"))
                (UserInterface|Viewport|AddtoViewport _returnvalue 0)
                (Default|IncreaseSanity PlayerRef 0.1)))))))))

(fn ConstructionScript)