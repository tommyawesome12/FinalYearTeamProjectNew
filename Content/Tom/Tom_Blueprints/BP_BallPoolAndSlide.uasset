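; Ball pool and slide prop actor that animates when the player enters its trigger box.
; Both skeletal meshes are stopped at BeginPlay.
; A Player-tagged overlap plays SkeletalMesh1 once, then after a short delay loops SkeletalMesh and reveals the Niagara effect.
; The construction script snaps that effect to the ParticleLocation socket on SkeletalMesh, keeping world rotation and scale.
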(event OnComponentBeginOverlap(Box)
  (params (OverlappedComponent :type Primitive%20Component%20Object%20Reference) (OtherActor :type Actor%20Object%20Reference) (OtherComp :type Primitive%20Component%20Object%20Reference) (OtherBodyIndex :type Integer) (bFromSweep :type Boolean) (SweepResult :type Hit%20Result%20Structure%20%28by%20ref%29))
  (if (Actor|ActorHasTag OtherActor "Player")
    (Audio|Components|Audio|Play (Variables|Default|GetSkeletalMesh1) false)
    (Utilities|FlowControl|Delay 2.0)
    (Audio|Components|Audio|Play (Variables|Default|GetSkeletalMesh) true)
    (Development|SetHiddeninGame (Variables|Default|GetNiagara) false false)))

(event EventBeginPlay
  (Audio|Components|Audio|Stop (Variables|Default|GetSkeletalMesh))
  (Audio|Components|Audio|Stop (Variables|Default|GetSkeletalMesh1)))

(event Collision|EventActorBeginOverlap
  (params (OtherActor :type Actor%20Object%20Reference)))

(event EventTick
  (params (DeltaSeconds :type Float%20%28single-precision%29)))

(fn ConstructionScript
  (Transformation|AttachComponentToComponent (Variables|Default|GetNiagara) (Variables|Default|GetSkeletalMesh) "ParticleLocation" "SnapToTarget" "KeepWorld" "KeepWorld" true))