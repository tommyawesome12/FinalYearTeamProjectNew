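; BP_Mother is the level-one goal actor that the player interacts with to win once all three items are collected.
; It caches BP_GM_Level1 on BeginPlay, and its ItemCollected event reveals a cone and spotlight marker when the count reaches three.
; Interact checks the game mode's collected count, then shows the win widget, pauses the game and switches to UI-only input with the mouse cursor.
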(event Custom|ItemCollected
  (params (NewParam :type Integer))
  ;[1 1 1] This gets triggered when all objects are collected
  (if (== NewParam 3)
    (Development|SetHiddeninGame (Variables|Default|GetCone) false false)
    (Development|SetHiddeninGame (Variables|Default|GetSpotLight) false false)))

(event Collision|EventActorBeginOverlap
  (params (OtherActor :type Actor%20Object%20Reference)))

(event EventTick
  (params (DeltaSeconds :type Float%20%28single-precision%29)))

(event EventInteract
  (params (PlayerRef :type BP%20Player%20Character%20Object%20Reference))
  (bind _returnvalue (Game|GetPlayerController 0))
  ;[1 1 1] make sure here that there is a check for if all ojectives have been collected
  (if (== (Variables|/Game/Tom/Tom_Blueprints/BP_GM_Level1.BP_GM_Level1_C|GetCollectedItems (Variables|Default|GetAs%20BP%20GM%20Level%201)) 3)
    (bind _returnvalue_2 (UserInterface|CreateWidget "/Game/Sharan/UI/BP_WIG_Win.BP_WIG_Win_C"))
    (UserInterface|Viewport|AddtoViewport _returnvalue_2 0)
    (Input|SetInputModeUIOnly _returnvalue _returnvalue_2 "DoNotLock" false)
    (Game|SetGamePaused true)
    (Variables|/Script/Engine.PlayerController|SetbShowMouseCursor _returnvalue true)))

(event EventBeginPlay
  (bind _asbp_gm_level_1 (Utilities|Casting|CastToBP_GM_Level1 (Game|GetGameMode)))
  (Variables|Default|SetAs%20BP%20GM%20Level%201 _asbp_gm_level_1))

(fn ConstructionScript)