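; BP_EventTrigger is a box trigger that fires random scare events when a Player-tagged actor enters it.
; On BeginPlay it builds buildup and release event pools from its enabled flags.
; Once the game mode's event cooldown is high enough, low player sanity selects a release jumpscare, otherwise a buildup event, each branch firing once.
; The random pick maps by array index to a game mode call, passing this trigger's referenced props.
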(event OnComponentBeginOverlap(Box)
  (params (OverlappedComponent :type Primitive%20Component%20Object%20Reference) (OtherActor :type Actor%20Object%20Reference) (OtherComp :type Primitive%20Component%20Object%20Reference) (OtherBodyIndex :type Integer) (bFromSweep :type Boolean) (SweepResult :type Hit%20Result%20Structure%20%28by%20ref%29))
  (bind _arrayofreleaseeventsforthistrigger (Variables|Default|GetArrayOfReleaseEventsForThisTrigger))
  (bind _game_mode_ref (Variables|Default|GetGame%20Mode%20Ref))
  (bind _arrayofeventsforthistrigger (Variables|Default|GetArrayOfEventsForThisTrigger))
  (bind _game_mode_ref_2 (Variables|Default|GetGame%20Mode%20Ref))
  ;[1 1 1] Selects Events to use
  (if (Actor|ActorHasTag OtherActor "Player")
    (if (>= (Variables|/Game/Tom/Tom_Blueprints/BP_GM_Level1.BP_GM_Level1_C|GetEventCooldown (Variables|Default|GetGame%20Mode%20Ref)) 2e+01)
      (if (<= (Variables|/Game/Tom/Tom_Blueprints/BP_PlayerCharacter.BP_PlayerCharacter_C|GetSanity (Variables|/Game/Tom/Tom_Blueprints/BP_GM_Level1.BP_GM_Level1_C|GetPlayerRef (Variables|Default|GetGame%20Mode%20Ref))) 0.45)
        (Utilities|FlowControl|DoOnce false
          (:Completed
            (Variables|Default|SetRandomNumberUsedForRelease (Utilities|Array|FindItem (Variables|Default|GetArrayOfPossibleReleaseEvents) (Utilities|Array|Get(acopy) _arrayofreleaseeventsforthistrigger (Math|Random|RandomIntegerinRange 0 (- (Utilities|Array|Length _arrayofreleaseeventsforthistrigger) 1)))))
            (Math|Integer|CompareInt (Variables|Default|GetRandomNumberUsedForRelease) 1
              (:==
                (Default|ShelfFallingOver _game_mode_ref (Variables|Default|GetRackToFall)))
              (:<
                (Default|HeadJumpatYou _game_mode_ref (Variables|Default|GetHeadToJumpAtYou))))))
        (else
          (Utilities|FlowControl|DoOnce false
            (:Completed
              (Variables|Default|SetRandomNumberUsed (Utilities|Array|FindItem (Variables|Default|GetArrayOfPossibleEvents) (Utilities|Array|Get(acopy) _arrayofeventsforthistrigger (Math|Random|RandomIntegerinRange 0 (- (Utilities|Array|Length _arrayofeventsforthistrigger) 1)))))
              (Math|Integer|CompareInt (Variables|Default|GetRandomNumberUsed) 1
                (:>
                  (Math|Integer|CompareInt (Variables|Default|GetRandomNumberUsed) 3
                    (:>
                      (Math|Integer|CompareInt (Variables|Default|GetRandomNumberUsed) 5
                        (:>
                          (Default|CallClothesFallEvent _game_mode_ref_2 (Variables|Default|GetClothesToFallWithEvent)))
                        (:==
                          (Default|CallLightFallEvent _game_mode_ref_2 (Variables|Default|GetLightToFallInvolvedWithEvent)))
                        (:<
                          (Default|CallCrunchSoundEvent _game_mode_ref_2))))
                    (:==
                      (Default|CallShakeRacksEvent _game_mode_ref_2 (Variables|Default|GetRacksInvolvedWithEvent)))
                    (:<
                      (Default|CallSingleRedLightEvent _game_mode_ref_2 (Variables|Default|GetLightToRedInvolvedWithEvent)))))
                (:==
                  (Default|CallBallRollEvent _game_mode_ref_2))
                (:<
                  (Default|CallCameraFallEvent _game_mode_ref_2 (Variables|Default|GetCamerasInvolvedInEvent)))))))))))

(event EventBeginPlay
  (bind _gamemoderef (Class|BPIGetGameMode|GetGameModeInterface(Message) (Game|GetGameMode)))
  (Variables|Default|SetGame%20Mode%20Ref _gamemoderef)
  (CallFunction|AddEventTypestoArray)
  (CallFunction|AddReleaseEventTypetoArray))

(event Collision|EventActorBeginOverlap
  (params (OtherActor :type Actor%20Object%20Reference)))

(event EventTick
  (params (DeltaSeconds :type Float%20%28single-precision%29)))

(fn ConstructionScript)

(fn AddEventTypestoArray
  (bind _possiblebuildupevents (Variables|Default|GetPossibleBuildupEvents))
  (bind _arrayofeventsforthistrigger (Variables|Default|GetArrayOfEventsForThisTrigger))
  (bind (_cameraevent _ballrolling _singlelightgoingred _multipleracksshaking _crunchingsoundaroundcorner _lightfalling _clothesfalling) (Utilities|Struct|BreakS_EventTypes _possiblebuildupevents))
  (Utilities|FlowControl|Sequence
    (:then_0
      (if _cameraevent
        (Utilities|Array|Add _arrayofeventsforthistrigger "Camera")))
    (:then_1
      (if _ballrolling
        (Utilities|Array|Add _arrayofeventsforthistrigger "Ball")))
    (:then_2
      (if _singlelightgoingred
        (Utilities|Array|Add _arrayofeventsforthistrigger "SingleLightRed")))
    (:then_3
      (if _multipleracksshaking
        (Utilities|Array|Add _arrayofeventsforthistrigger "RacksShake")))
    (:then_4
      (if _crunchingsoundaroundcorner
        (Utilities|Array|Add _arrayofeventsforthistrigger "CrunchSound")))
    (:then_5
      (if _lightfalling
        (Utilities|Array|Add _arrayofeventsforthistrigger "LightFalling")))
    (:then_6
      (if _clothesfalling
        (Utilities|Array|Add _arrayofeventsforthistrigger "ClothesFalling")))))

(fn AddReleaseEventTypetoArray
  (bind _possiblereleaseevents (Variables|Default|GetPossibleReleaseEvents))
  (bind _arrayofreleaseeventsforthistrigger (Variables|Default|GetArrayOfReleaseEventsForThisTrigger))
  (bind (_headjumpscare _rackfallover) (Utilities|Struct|BreakS_TensionReleaseEventTypes _possiblereleaseevents))
  (Utilities|FlowControl|Sequence
    (:then_0
      (if _headjumpscare
        (Utilities|Array|Add _arrayofreleaseeventsforthistrigger "HeadJumpScare")))
    (:then_1
      (if _rackfallover
        (Utilities|Array|Add _arrayofreleaseeventsforthistrigger "ShelfFallOver")))))

(fn GetGameModeInterface
  (return 0))