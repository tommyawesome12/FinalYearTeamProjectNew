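; First-person player character for a horror level with sanity, stamina-limited sprinting, objective pickups and a toggleable shopping list.
; Tick drives stamina, sanity recovery while hiding, footsteps and speed-based camera-shake headbob.
; Sanity changes update BP_GM_Level1 and chromatic aberration alongside an outline post-process.
; Events handle line-trace interaction, reassurance-area UI, death screen, fade-to-black flicker and roll correction, while jump input is unwired.
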(event Custom|StartStaminaRegen
  ;[1 1 1] Stamina Regen Mechanic
  (Utilities|FlowControl|RetriggerableDelay (Variables|Default|GetStaminaRegenCooldown))
  (Variables|Default|SetCanRegenStamina true))

(event Custom|UpdatePostProcess
  (params (SanityValue :type Float%20%28double-precision%29))
  ;[1 1 1] Adds chromatic abberration to player screen
  (Variables|/Script/Engine.PostProcessComponent|SetSettings (Variables|Default|GetPostProcess) (Utilities|Struct|MakePostProcessSettings "AEM_Manual" (* (- 1.0 SanityValue) (Variables|Default|GetMaxChromaticAbberration)) (Variables|Default|GetExposure%20Compensation) 1.0 1.0 2e+01 2e+01 (Utilities|Struct|MakeWeightedBlendables (Utilities|Array|MakeArray (Utilities|Struct|MakeWeightedBlendable 1.0 "/Game/James/PP_OutlineShader_Inst.PP_OutlineShader_Inst"))))))

(event Custom|PlayerDeath
  (bind _returnvalue (Game|GetPlayerController 0))
  ;[1 1 1] Player death screen
  (bind _returnvalue_2 (UserInterface|CreateWidget "/Game/Sharan/UI/BP_WIG_Death.BP_WIG_Death_C"))
  (UserInterface|Viewport|AddtoViewport _returnvalue_2 0)
  (Game|SetGamePaused true)
  (Variables|/Script/Engine.PlayerController|SetbShowMouseCursor _returnvalue true)
  (Input|SetInputModeUIOnly _returnvalue _returnvalue_2 "DoNotLock" false))

(event Custom|SmoothOrientation
  (params (NewControlRotation :type Rotator))
  ;[1 1 1] Smoothing orientation
  (if (or (!= (.roll (Pawn|GetControlRotation (Game|GetPlayerController 0) :!class /Script/Engine.Controller)) 0.0) (!= (.roll (Transformation|GetWorldRotation (Variables|Collision|GetCapsuleComponent))) 0.0))
    (Variables|Default|SetInitialControlRotation (Pawn|GetControlRotation (Game|GetPlayerController 0) :!class /Script/Engine.Controller))
    (Variables|Default|SetInitialWorldRotation (Transformation|GetWorldRotation (Variables|Collision|GetCapsuleComponent)))
    (bind _alpha (Timeline|Rotate PlayFromStart)
      (:Update
        (Pawn|SetControlRotation (Game|GetPlayerController 0) (Math|Interpolation|Ease "EaseInOut" _alpha (Variables|Default|GetInitialControlRotation) (Math|Rotator|MakeRotator 0.0 (.Pitch (Math|Rotator|BreakRotator (Variables|Default|GetInitialControlRotation))) (.Yaw (Math|Rotator|BreakRotator (Variables|Default|GetInitialControlRotation)))) true))
        (Transformation|SetWorldRotation (Variables|Collision|GetCapsuleComponent) (Math|Interpolation|Ease "EaseInOut" _alpha (Variables|Default|GetInitialWorldRotation) (Math|Rotator|MakeRotator 0.0 0.0 0.0) true) false false)))))

(event Custom|FadeToBlack
  ;[1 1 1] Fading to black for light flickering
  (if (Variables|Default|GetCanFadeToBlack)
    (if (Variables|/Game/Tom/Tom_Blueprints/BP_GM_Level1.BP_GM_Level1_C|GetInBadPlace (Variables|Default|GetAs%20BP%20GM%20Level%201))
      (bind _newtrack_0 (Timeline|Timeline PlayFromStart)
        (:Update
          (Variables|/Script/Engine.CameraComponent|SetPostProcessSettings (Variables|Default|GetCamera) (Utilities|Struct|MakePostProcessSettings "AEM_Manual" (* _newtrack_0 (Variables|Default|GetExposure%20Compensation)))))))))

(event Custom|Headbob
  (bind _returnvalue (Transformation|GetVelocity))
  (bind _returnvalue_2 (Game|GetPlayerController 0))
  (bind _returnvalue_3 (Math|Vector|VectorLength _returnvalue))
  ;[0.2812 0.9901 1] Headbob
  (if (and (Character|CanJump) (> _returnvalue_3 0.0))
    (if (< _returnvalue_3 3e+02)
      (Game|Feedback|ClientStartCameraShake _returnvalue_2 "/Game/Sharan/Blueprints/BP_WalkCamerashake.BP_WalkCamerashake_C" 1.0 "CameraLocal" "0, 0, 0")
      (else
        (Game|Feedback|ClientStartCameraShake _returnvalue_2 "/Game/Sharan/Blueprints/BP_SprintCamerashake.BP_SprintCamerashake_C" 1.0 "CameraLocal" "0, 0, 0")))
    (else
      (Game|Feedback|ClientStartCameraShake _returnvalue_2 "/Game/Sharan/Blueprints/BP_IdleCamerashake.BP_IdleCamerashake_C" 1.0 "CameraLocal" "0, 0, 0"))))

(event Input|EnhancedActionEvents|EnhancedInputActionIA_Move
  (params (ActionValue :type Vector%202D%20Structure) (ElapsedSeconds :type Float%20%28double-precision%29) (TriggeredSeconds :type Float%20%28double-precision%29) (InputAction :type Input%20Action%20Object%20Reference :default "/Game/FirstPerson/Input/Actions/IA_Move.IA_Move"))
  ;[1 1 1] Movement mechanics
  (Pawn|Input|AddMovementInput (Transformation|GetActorRightVector) (.x ActionValue) false)
  (Pawn|Input|AddMovementInput (Transformation|GetActorForwardVector) (.y ActionValue) false))

(event Input|EnhancedActionEvents|EnhancedInputActionIA_LookAround
  (params (ActionValue :type Vector%202D%20Structure) (ElapsedSeconds :type Float%20%28double-precision%29) (TriggeredSeconds :type Float%20%28double-precision%29) (InputAction :type Input%20Action%20Object%20Reference :default "/Game/Tom/PlayerInputs/InputActions/IA_LookAround.IA_LookAround"))
  ;[1 1 1] Look Around Mechanics
  (Pawn|Input|AddControllerYawInput (.x ActionValue))
  (bind _result (Math|Float|NegateFloat (.y ActionValue))
    (:%20%20
      (Pawn|Input|AddControllerPitchInput _result))))

(event Input|EnhancedActionEvents|EnhancedInputActionIA_Sprint
  (params (ActionValue :type Boolean) (ElapsedSeconds :type Float%20%28double-precision%29) (TriggeredSeconds :type Float%20%28double-precision%29) (InputAction :type Input%20Action%20Object%20Reference :default "/Game/Tom/PlayerInputs/InputActions/IA_Sprint.IA_Sprint"))
  ;[1 1 1] Sprinting mechanic
  (:Triggered
    (if (> (Math|Vector|VectorLength (Transformation|GetVelocity)) 0.0) :!label _label
      (if (> (Variables|Default|GetStamina) 0.0)
        (CallFunction|StartSprint)
        (else
          (CallFunction|FallOver)))))
  (:Started
    (goto _label))
  (:Completed
    (CallFunction|StopSprint)))

(event Input|EnhancedActionEvents|EnhancedInputActionIA_PlayerJump
  (params (ActionValue :type Boolean) (ElapsedSeconds :type Float%20%28double-precision%29) (TriggeredSeconds :type Float%20%28double-precision%29) (InputAction :type Input%20Action%20Object%20Reference :default "/Game/Tom/PlayerInputs/InputActions/IA_PlayerJump.IA_PlayerJump"))
  ;[1 1 1] Jumping
)

(event Input|EnhancedActionEvents|EnhancedInputActionIA_Interact
  (params (ActionValue :type Boolean) (ElapsedSeconds :type Float%20%28double-precision%29) (TriggeredSeconds :type Float%20%28double-precision%29) (InputAction :type Input%20Action%20Object%20Reference :default "/Game/Tom/PlayerInputs/InputActions/IA_Interact.IA_Interact"))
  (bind _camera (Variables|Default|GetCamera))
  (bind _returnvalue (Transformation|GetWorldLocation _camera))
  ;[1 1 1] InteractionInputLinetrace
  (:Started
    (bind _outhit (Collision|LineTraceByChannel _returnvalue (+ _returnvalue (* (Math|Vector|GetForwardVector _camera) 1e+08)) "TraceTypeQuery1" false 0 "None"))
    (if (Utilities|DoesObjectImplementInterface (.HitActor (Collision|BreakHitResult _outhit)) "/Game/Tom/Tom_Blueprints/BPI_Interact.BPI_Interact_C")
      (if (< (.Distance (Collision|BreakHitResult _outhit)) 3e+02)
        (if (Actor|ActorHasTag (.HitActor (Collision|BreakHitResult _outhit)) "Objective")
          (bind _result (Math|Integer|IncrementInt (Variables|Default|GetCollectedObjectives))
            (:%20%20
              (Class|BPIInteract|Interact(Message) (.HitActor (Collision|BreakHitResult _outhit)))
              (Default|RecordPickup (Variables|Default|GetAs%20BP%20GM%20Level%201) _result))))))))

(event Input|EnhancedActionEvents|EnhancedInputActionIA_OpenList
  (params (ActionValue :type Boolean) (ElapsedSeconds :type Float%20%28double-precision%29) (TriggeredSeconds :type Float%20%28double-precision%29) (InputAction :type Input%20Action%20Object%20Reference :default "/Game/Tom/PlayerInputs/InputActions/IA_OpenList.IA_OpenList"))
  ;[1 1 1] Open List UI
  (:Started
    (if (Variables|Default|GetShoppingListOpen)
      (Widget|RemovefromParent (Variables|Default|GetShoppingListRef))
      (Variables|Default|SetShoppingListOpen false)
      (else
        (Utilities|IsValid 0
          (:Is%20Valid
            _)
          (:Is%20Not%20Valid
            (bind _returnvalue (UserInterface|CreateWidget "/Game/Sharan/UI/BP_WIG_ShoppingList.BP_WIG_ShoppingList_C" (Game|GetPlayerController 0)))
            (Variables|Default|SetShoppingListRef _returnvalue)))
        (UserInterface|Viewport|AddtoViewport (Variables|Default|GetShoppingListRef) 0)
        (Variables|Default|SetShoppingListOpen true)))))

(event EventBeginPlay
  (bind _returnvalue (UserInterface|CreateWidget "/Game/Sharan/UI/BP_WIG_Power.BP_WIG_Power_C"))
  (UserInterface|Viewport|AddtoViewport _returnvalue 0)
  (bind _asbp_gm_level_1 (Utilities|Casting|CastToBP_GM_Level1 (Game|GetGameMode)))
  (Variables|Default|SetAs%20BP%20GM%20Level%201 _asbp_gm_level_1)
  (bind _returnvalue_2 (UserInterface|CreateWidget "/Game/Tom/TempUI/BP_WJ_Subtitles.BP_WJ_Subtitles_C"))
  (UserInterface|Viewport|AddtoViewport _returnvalue_2 0)
  (CallFunction|UpdatePostProcess (Variables|Default|GetSanity))
  (bind _returnvalue_3 (UserInterface|CreateWidget "/Game/Tom/TempUI/BP_WJ_Crosshair.BP_WJ_Crosshair_C"))
  (UserInterface|Viewport|AddtoViewport _returnvalue_3 0)
  (Rendering|SetVisibility (Variables|Default|GetNS_Speeding) false false))

(event Collision|EventActorBeginOverlap
  (params (OtherActor :type Actor%20Object%20Reference)))

(event EventReassuranceAreaEnter
  (params (ReassuranceAreaRef :type BP%20Reassurance%20Area%20Object%20Reference))
  ;[1 1 1] Update duration of reassurance area
  (Utilities|IsValid (Variables|Default|GetReassuranceZoneUIRef)
    (:Is%20Valid
      _)
    (:Is%20Not%20Valid
      (bind _returnvalue (UserInterface|CreateWidget "/Game/Tom/TempUI/BP_WJ_ReassuranceAreaDuration.BP_WJ_ReassuranceAreaDuration_C"))
      (Variables|Default|SetReassuranceZoneUIRef _returnvalue)))
  (UserInterface|Viewport|AddtoViewport (Variables|Default|GetReassuranceZoneUIRef) 0)
  (Variables|/Game/Tom/TempUI/BP_WJ_ReassuranceAreaDuration.BP_WJ_ReassuranceAreaDuration_C|SetDurationDecimal (Variables|Default|GetReassuranceZoneUIRef) (- 1.0 (/ (Variables|/Game/Tom/Tom_Blueprints/BP_ReassuranceArea.BP_ReassuranceArea_C|GetTimer ReassuranceAreaRef) (Variables|/Game/Tom/Tom_Blueprints/BP_ReassuranceArea.BP_ReassuranceArea_C|GetDuration ReassuranceAreaRef)))))

(event EventTick
  (params (DeltaSeconds :type Float%20%28single-precision%29))
  (Utilities|FlowControl|Sequence
    (:then_0
      ;[1 1 1] StaminaDecreasing and increaseing
      (if (Variables|Default|GetIsHiding)
        (if (< (Variables|Default|GetSanity) 0.7)
          (CallFunction|IncreaseSanity (/ DeltaSeconds (Variables|Default|GetSanityIncreaseTime))))))
    (:then_1
      (if (Variables|Default|GetIsSprinting)
        (CallFunction|DecreaseStamina (/ DeltaSeconds (Variables|Default|GetSprintDuration)))))
    (:then_2
      (if (Variables|Default|GetCanRegenStamina)
        (CallFunction|IncreaseStamina (/ DeltaSeconds (Variables|Default|GetStaminaRegenTime)))))
    (:then_3
      ;[1 1 1] Stamina Regen Mechanic
      (if (> (Math|Vector|VectorLength (Transformation|GetVelocity)) 0.0)
        (Utilities|FlowControl|DoOnce false :!label _label
          (:Completed
            (Audio|PlaySound2D "/Game/Sharan/Audio/SoundCues/FootStepsIdle_Cue.FootStepsIdle_Cue" 1.0 1.0 0.0 0 0)
            (Utilities|FlowControl|Delay 0.4)
            (goto _label Reset)))))
    (:then_4
      (CallFunction|Headbob))))

(event EventReassuranceAreaExit
  (bind _reassurancezoneuiref (Variables|Default|GetReassuranceZoneUIRef))
  ;[1 1 1] Closes reassurance area ui
  (Utilities|IsValid _reassurancezoneuiref
    (:Is%20Valid
      (Widget|RemovefromParent _reassurancezoneuiref))))

(fn ConstructionScript)

(fn StartSprint
  (Variables|/Script/Engine.CharacterMovementComponent|SetMaxWalkSpeed (Variables|Character|GetCharacterMovement) (Variables|Default|GetRunSpeed))
  (Variables|Default|SetIsSprinting true))

(fn StopSprint
  (Variables|/Script/Engine.CharacterMovementComponent|SetMaxWalkSpeed (Variables|Character|GetCharacterMovement) (Variables|Default|GetWalkSpeed))
  (Variables|Default|SetIsSprinting false))

(fn FallOver
  (CallFunction|StopSprint))

(fn IncreaseStamina
  (params (IncreaseAmount :type Float%20%28double-precision%29))
  (if (< (Variables|Default|GetStamina) 1.0)
    (Variables|Default|SetStamina (+ (Variables|Default|GetStamina) IncreaseAmount))))

(fn DecreaseStamina
  (params (DecreaseAmount :type Float%20%28double-precision%29))
  (if (> (Variables|Default|GetStamina) 0.0)
    (Variables|Default|SetStamina (- (Variables|Default|GetStamina) DecreaseAmount))
    (Variables|Default|SetCanRegenStamina false)
    (CallFunction|StartStaminaRegen)
    (else
      (CallFunction|FallOver))))

(fn IncreaseSanity
  (params (IncreaseAmount :type Float%20%28double-precision%29))
  (if (< (Variables|Default|GetSanity) 1.0)
    (Variables|Default|SetSanity (+ (Variables|Default|GetSanity) IncreaseAmount)))
  (Default|UpdateSanity (Variables|Default|GetAs%20BP%20GM%20Level%201) (Variables|Default|GetSanity))
  (CallFunction|UpdatePostProcess (Variables|Default|GetSanity)))

(fn DecreaseSanity
  (params (DecreaseAmount :type Float%20%28double-precision%29))
  (if (> (Variables|Default|GetSanity) 0.0)
    (Variables|Default|SetSanity (- (Variables|Default|GetSanity) (* DecreaseAmount (Math|Float|Clamp(Float) (* (Variables|Default|GetSanity) 2.0) 1.0 2.0)))))
  (Default|UpdateSanity (Variables|Default|GetAs%20BP%20GM%20Level%201) (Variables|Default|GetSanity))
  (CallFunction|UpdatePostProcess (Variables|Default|GetSanity)))