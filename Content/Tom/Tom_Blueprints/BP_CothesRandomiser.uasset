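; A spline placement actor, named as a clothes randomiser, that lays copies of a chosen mesh along a spline.
; The construction script adds an instanced static mesh component and spaces NumberOfItems instances evenly by spline length, each rotated to the local tangent.
; Nothing is randomised yet: the UpdateClothes event takes a SanityValue but is empty, and the Material variable is unused.
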(event Custom|UpdateClothes
  (params (SanityValue :type Float%20%28double-precision%29)))

(event EventBeginPlay)

(event Collision|EventActorBeginOverlap
  (params (OtherActor :type Actor%20Object%20Reference)))

(event EventTick
  (params (DeltaSeconds :type Float%20%28single-precision%29)))

(fn ConstructionScript
  (bind _spline (Variables|Default|GetSpline))
  (bind _returnvalue (AddComponent|AddInstancedStaticMeshComponent false))
  (Components|StaticMesh|SetStaticMesh _returnvalue (Variables|Default|GetMesh))
  (for _index (range 0 (- (Variables|Default|GetNumberOfItems) 1))
    (Components|InstancedStaticMesh|AddInstance _returnvalue (Math|Transform|MakeTransform (Spline|GetLocationatDistanceAlongSpline _spline (* _index (/ (Spline|GetSplineLength _spline) (Variables|Default|GetNumberOfItems))) "Local") (Math|Conversions|RotationFromXVector (Spline|GetTangentatDistanceAlongSpline (Variables|Default|GetSpline) (* _index (/ (Spline|GetSplineLength _spline) (Variables|Default|GetNumberOfItems))) "Local")) "1.000000,1.000000,1.000000") false)))