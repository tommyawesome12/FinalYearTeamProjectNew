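; Folded trousers prop that gets a random colour and can shift its tint according to a sanity value.
; The construction script creates a dynamic material with a random RandomColour and applies it to the mesh, without storing it in the DynamicMaterialInstance variable.
; UpdateTexture sets RandomColour on that variable, blending from grey towards black as SanityValue rises above 0.5.
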(event Custom|UpdateTexture
  (params (SanityValue :type Float%20%28double-precision%29))
  (if true
    (Rendering|Material|SetVectorParameterValue (Variables|Default|GetDynamicMaterialInstance) "RandomColour" (Math|Color|Lerp(LinearColor) :A "(R=0.375000,G=0.375000,B=0.375000,A=1.000000)" :Alpha (Math|Float|Clamp(Float) (- SanityValue 0.5))) :!class /Script/Engine.MaterialInstanceDynamic)))

(event EventBeginPlay)

(event Collision|EventActorBeginOverlap
  (params (OtherActor :type Actor%20Object%20Reference)))

(fn ConstructionScript
  (bind _returnvalue (Rendering|Material|CreateDynamicMaterialInstance (Variables|Default|GetMaterialInstace) "None" "None" :!class /Script/Engine.KismetMaterialLibrary))
  (bind _output_get (Variables|Default|SetLinearColour (Utilities|Struct|MakeLinearColor (Math|Random|RandomFloat) (Math|Random|RandomFloat) (Math|Random|RandomFloat) 1.0)))
  (Rendering|Material|SetVectorParameterValue _returnvalue "RandomColour" _output_get :!class /Script/Engine.MaterialInstanceDynamic)
  (Rendering|Material|SetMaterial (Variables|Default|GetStaticMesh) 0 _returnvalue))