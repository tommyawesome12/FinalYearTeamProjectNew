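; Jump-scare head actor that launches itself at the player when its JumpAtPlayer event is called.
; JumpAtPlayer plays a growl, waits briefly, then sets ProjectileMovement velocity toward the player camera, found through a Game Mode interface reference cached at BeginPlay.
; Once jumping, it turns to face the player every tick.
; A sphere overlap with the Player-tagged actor during the jump triggers the player's fade to black, then destroys the head.
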(event OnComponentBeginOverlap(Sphere)
  (params (OverlappedComponent :type Primitive%20Component%20Object%20Reference) (OtherActor :type Actor%20Object%20Reference) (OtherComp :type Primitive%20Component%20Object%20Reference) (OtherBodyIndex :type Integer) (bFromSweep :type Boolean) (SweepResult :type Hit%20Result%20Structure%20%28by%20ref%29))
  (if (Actor|ActorHasTag OtherActor "Player")
    (if (Variables|Default|GetCanJump)
      (Default|FadetoBlack (Variables|/Game/Tom/Tom_Blueprints/BP_GM_Level1.BP_GM_Level1_C|GetPlayerRef (Variables|Default|GetGame%20Mode%20Ref)))
      (Utilities|FlowControl|Delay 0.5)
      (Actor|DestroyActor))))

(event Custom|JumpAtPlayer
  (Development|PrintString "jump")
  (Audio|PlaySound2D "/Game/Sharan/Audio/AudioHorror/LongGrowl.LongGrowl" 1.0 1.0 0.0 0 0)
  (Utilities|FlowControl|Delay 0.5)
  (Variables|Default|SetCanJump true)
  (Variables|/Script/Engine.MovementComponent|SetVelocity (Variables|Default|GetProjectileMovement) (* (Math|Vector|Normalize (- (Transformation|GetWorldLocation (Variables|/Game/Tom/Tom_Blueprints/BP_PlayerCharacter.BP_PlayerCharacter_C|GetCamera (Variables|/Game/Tom/Tom_Blueprints/BP_GM_Level1.BP_GM_Level1_C|GetPlayerRef (Variables|Default|GetGame%20Mode%20Ref)))) (Transformation|GetActorLocation))) 2e+03)))

(event EventBeginPlay
  (bind _gamemoderef (Class|BPIGetGameMode|GetGameModeInterface(Message) (Game|GetGameMode)))
  (Variables|Default|SetGame%20Mode%20Ref _gamemoderef))

(event Collision|EventActorBeginOverlap
  (params (OtherActor :type Actor%20Object%20Reference)))

(event EventTick
  (params (DeltaSeconds :type Float%20%28single-precision%29))
  (if (Variables|Default|GetCanJump)
    (Transformation|SetActorRotation (Math|Rotator|FindLookatRotation (Transformation|GetActorLocation) (Transformation|GetActorLocation (Game|GetPlayerCharacter 0))))))

(fn ConstructionScript)