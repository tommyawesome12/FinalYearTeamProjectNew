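; BP_PickupBase is a pickup base Blueprint that provides a configurable appearance and contains no collection logic in its graphs.
; The construction script applies the MeshToUse and MaterialToUse variables to the Sphere1 static mesh component, setting material slot 0.
; The UpdateLooks event repeats the same assignment so the look can be refreshed after construction.
; BeginPlay is empty, and the overlap and tick events are disabled placeholders.
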(event Custom|UpdateLooks
  (bind _sphere1 (Variables|Default|GetSphere1))
  (Components|StaticMesh|SetStaticMesh _sphere1 (Variables|Default|GetMeshToUse))
  (Rendering|Material|SetMaterial _sphere1 0 (Variables|Default|GetMaterialToUse)))

(event EventBeginPlay)

(event Collision|EventActorBeginOverlap
  (params (OtherActor :type Actor%20Object%20Reference)))

(event EventTick
  (params (DeltaSeconds :type Float%20%28single-precision%29)))

(fn ConstructionScript
  (bind _sphere1 (Variables|Default|GetSphere1))
  (Components|StaticMesh|SetStaticMesh _sphere1 (Variables|Default|GetMeshToUse))
  (Rendering|Material|SetMaterial _sphere1 0 (Variables|Default|GetMaterialToUse)))