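; BP_Lights is a spotlight actor that flickers at low sanity, can fall, and hosts a red light event with whispering audio.
; UpdateLighting sets the flicker light function and flag from the sanity value, while Fall hides the actor and spawns a BP_LightProjectile.
; TurnLightRed arms a Tick check that sphere-traces at the Arrow's line-trace hit until it finds the Player, then restores the colour and notifies the game mode.
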(event Custom|Fall
  (Rendering|SetActorHiddenInGame true)
  (Game|SpawnActorfromClass "/Game/Tom/Tom_Blueprints/BP_LightProjectile.BP_LightProjectile_C" (Math|Transform|MakeTransform (- (Transformation|GetActorLocation) "0.000000,0.000000,100.000000") "1.000000,0.000000,0.000000" "1.000000,1.000000,1.000000") "Undefined" "MultiplyWithRoot" 0 0))

(event Custom|TurnLightRed
  (bind _spotlight (Variables|Default|GetSpotLight))
  (bind _cone (Variables|Default|GetCone))
  (Audio|Components|Audio|SetVolumeMultiplier (Variables|Default|GetWhispers_Cue) 1.0 :!class /Script/Engine.AudioComponent)
  (Rendering|Components|Light|SetLightColor _spotlight "(R=1.000000,G=0.000000,B=0.004000,A=1.000000)" true)
  (Rendering|Components|Light|SetLightFunctionMaterial _spotlight "/Game/Sharan/Materials/M_LightFlicker2.M_LightFlicker2")
  (Variables|Default|SetSingleRedLightEvent true)
  (Rendering|SetVisibility _cone true false)
  (Development|SetHiddeninGame _cone false false))

(event Custom|UpdateLighting
  (params (SanityValue :type Float%20%28double-precision%29))
  (bind _spotlight (Variables|Default|GetSpotLight))
  (Utilities|FlowControl|Sequence
    (:then_0
      (if (< SanityValue 0.3)
        (Rendering|Components|Light|SetLightFunctionMaterial _spotlight "/Game/Sharan/Materials/M_LightFlicker2.M_LightFlicker2")
        (else
          (Rendering|Components|Light|SetLightFunctionMaterial _spotlight 0))))
    (:then_1
      (if (< SanityValue 0.1)
        (Variables|Default|SetLightFlickering true)
        (else
          (Variables|Default|SetLightFlickering false))))))

(event EventBeginPlay
  (bind _gamemoderef (Class|BPIGetGameMode|GetGameModeInterface(Message) (Game|GetGameMode)))
  (Variables|Default|SetGame%20Mode%20Ref _gamemoderef)
  (Audio|Components|Audio|SetVolumeMultiplier (Variables|Default|GetWhispers_Cue) 0.0 :!class /Script/Engine.AudioComponent))

(event Collision|EventActorBeginOverlap
  (params (OtherActor :type Actor%20Object%20Reference)))

(event EventTick
  (params (DeltaSeconds :type Float%20%28single-precision%29))
  (bind _cone (Variables|Default|GetCone))
  (bind _spotlight (Variables|Default|GetSpotLight))
  (bind _arrow (Variables|Default|GetArrow))
  (bind _actorstoignore (Variables|Default|GetActorsToIgnore))
  (if (Variables|Default|GetSingleRedLightEvent)
    (bind _outhit (Collision|LineTraceByChannel (Transformation|GetWorldLocation _arrow) (* (Math|Vector|GetForwardVector _arrow) 1e+07) "TraceTypeQuery4" false 0 "None"))
    (Utilities|Array|Add _actorstoignore (.HitActor (Collision|BreakHitResult _outhit)))
    (Variables|Default|SetImpactLocation (.Location (Collision|BreakHitResult _outhit)))
    (bind (_outhit_2 _returnvalue) (Collision|SphereTraceByChannel (.Location (Collision|BreakHitResult _outhit)) (.Location (Collision|BreakHitResult _outhit)) 1e+02 "TraceTypeQuery4" false _actorstoignore "None"))
    (if _returnvalue
      (if (Actor|ActorHasTag (.HitActor (Collision|BreakHitResult _outhit_2)) "Player")
        (Variables|Default|SetSingleRedLightEvent false)
        (Rendering|Components|Light|SetLightColor _spotlight "(R=0.792157,G=0.800000,B=1.000000,A=1.000000)" true)
        (Rendering|Components|Light|SetLightFunctionMaterial _spotlight "/Game/Sharan/Materials/M_LightFlicker2.M_LightFlicker2")
        (Default|FinishSingleRedLightEvent (Variables|Default|GetGame%20Mode%20Ref))
        (Rendering|SetVisibility _cone false false)
        (Development|SetHiddeninGame _cone true false)
        (else
          (Audio|Components|Audio|SetVolumeMultiplier (Variables|Default|GetWhispers_Cue) 0.0 :!class /Script/Engine.AudioComponent))))))

(fn ConstructionScript)

(fn TurnLightOff
  (Rendering|Components|Light|SetIntensity (Variables|Default|GetSpotLight) 0.0)
  (Variables|Default|SetLightTimer 0.0)
  (Variables|Default|SetLightOn false))

(fn TurnLighton
  (Rendering|Components|Light|SetIntensity (Variables|Default|GetSpotLight) 7.5e+03)
  (Variables|Default|SetLightTimer 0.0)
  (Variables|Default|SetLightOn false))