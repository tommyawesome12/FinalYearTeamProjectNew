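; Scare-style silhouette event actor with a Cube, a Head and a SpotLight, whose figure vanishes under a flickering light.
; The MakeInvisible custom event applies a flicker light function material, then after a short delay hides both meshes and turns the light white.
; A second delay clears the light function to end the flicker, which masks the disappearance.
; Nothing inside the Blueprint triggers the event.
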(event Custom|MakeInvisible
  (bind _spotlight (Variables|Default|GetSpotLight))
  (Rendering|Components|Light|SetLightFunctionMaterial (Variables|Default|GetSpotLight) "/Game/Sharan/Materials/M_LightFlicker2.M_LightFlicker2")
  (Utilities|FlowControl|Delay 0.5)
  (Development|SetHiddeninGame (Variables|Default|GetCube) true false)
  (Rendering|SetVisibility (Variables|Default|GetHead) false false)
  (Rendering|Components|Light|SetLightColor _spotlight "(R=1.000000,G=1.000000,B=1.000000,A=1.000000)" true)
  (Utilities|FlowControl|Delay 0.5)
  (Rendering|Components|Light|SetLightFunctionMaterial _spotlight 0))

(event EventBeginPlay)

(event Collision|EventActorBeginOverlap
  (params (OtherActor :type Actor%20Object%20Reference)))

(event EventTick
  (params (DeltaSeconds :type Float%20%28single-precision%29)))

(fn ConstructionScript)