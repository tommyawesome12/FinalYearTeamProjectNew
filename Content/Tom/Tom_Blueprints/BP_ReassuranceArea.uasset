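; Limited-duration safe area for Level 1 that reassures the player and holds off the RBP_Mannequine1 mannequins.
; While the player overlaps the box, a per-tick line trace sets the game mode's InBadPlace flag, and safe time counts toward Duration.
; In-range ticks also send mannequins home and stop them, while blocked traces or leaving restart their logic.
; On expiry it flags InBadPlace and destroys itself.
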(event OnComponentBeginOverlap(Box)
  (params (OverlappedComponent :type Primitive%20Component%20Object%20Reference) (OtherActor :type Actor%20Object%20Reference) (OtherComp :type Primitive%20Component%20Object%20Reference) (OtherBodyIndex :type Integer) (bFromSweep :type Boolean) (SweepResult :type Hit%20Result%20Structure%20%28by%20ref%29))
  ;[1 1 1] Chekcs if player is inside colision or not
  (Variables|Default|SetTargetPlayer OtherActor)
  (if (Actor|ActorHasTag OtherActor "Player")
    (Variables|Default|SetplayerInRange true)))

(event OnComponentEndOverlap(Box)
  (params (OverlappedComponent :type Primitive%20Component%20Object%20Reference) (OtherActor :type Actor%20Object%20Reference) (OtherComp :type Primitive%20Component%20Object%20Reference) (OtherBodyIndex :type Integer))
  ;[1 1 1] Chekcs if player is inside colision or not
  (Variables|Default|SetTargetPlayer 0)
  (if (Actor|ActorHasTag OtherActor "Player")
    (Variables|Default|SetplayerInRange false)
    (Variables|/Game/Tom/Tom_Blueprints/BP_GM_Level1.BP_GM_Level1_C|SetInBadPlace (Variables|Default|GetGameModeRef) true)
    (Class|BPIReassuranceInterface|ReassuranceAreaExit(Message) OtherActor)
    (bind _outactors (Actor|GetAllActorsOfClass "/Game/Sharan/Blueprints/RBP_Mannequine1.RBP_Mannequine1_C"))
    (for _array_element _outactors
      (Default|StartLogic _array_element))))

(event EventBeginPlay
  (bind _actors_to_ignore (Variables|Default|GetActors%20to%20Ignore))
  ;[1 1 1] Sets variable
  (bind _asbp_gm_level_1 (Utilities|Casting|CastToBP_GM_Level1 (Game|GetGameMode)))
  (Variables|Default|SetGameModeRef _asbp_gm_level_1)
  (Utilities|Array|Add _actors_to_ignore self)
  (Utilities|Array|Add _actors_to_ignore (Game|GetPlayerCharacter 0)))

(event Collision|EventActorBeginOverlap
  (params (OtherActor :type Actor%20Object%20Reference))
  ;[1 1 1] Checks that there is no wall in the way
)

(event EventTick
  (params (DeltaSeconds :type Float%20%28single-precision%29))
  (bind _gamemoderef (Variables|Default|GetGameModeRef))
  (if (>= (Variables|Default|GetTimer) (Variables|Default|GetDuration))
    ;[1 1 1] Checks that there is no wall in the way
    (Variables|/Game/Tom/Tom_Blueprints/BP_GM_Level1.BP_GM_Level1_C|SetInBadPlace (Variables|Default|GetGameModeRef) true)
    (Actor|DestroyActor)
    (elif (Variables|Default|GetplayerInRange)
      (Utilities|FlowControl|Sequence
        (:then_0
          (bind _returnvalue (Collision|LineTraceByChannel (Transformation|GetActorLocation) (Transformation|GetActorLocation (Game|GetPlayerCharacter 0)) "TraceTypeQuery3" false (Variables|Default|GetActors%20to%20Ignore) "None"))
          (if _returnvalue
            (Variables|/Game/Tom/Tom_Blueprints/BP_GM_Level1.BP_GM_Level1_C|SetInBadPlace _gamemoderef true)
            (bind _outactors (Actor|GetAllActorsOfClass "/Game/Sharan/Blueprints/RBP_Mannequine1.RBP_Mannequine1_C"))
            (for _array_element _outactors
              (Default|StartLogic _array_element))
            (else
              (Variables|/Game/Tom/Tom_Blueprints/BP_GM_Level1.BP_GM_Level1_C|SetInBadPlace _gamemoderef false)
              (Class|BPIReassuranceInterface|ReassuranceAreaEnter(Message) (Variables|Default|GetTargetPlayer) self))))
        (:then_1
          ;[1 1 1] timer for duraion
          (if (not (Variables|/Game/Tom/Tom_Blueprints/BP_GM_Level1.BP_GM_Level1_C|GetInBadPlace (Variables|Default|GetGameModeRef)))
            (Variables|Default|SetTimer (+ DeltaSeconds (Variables|Default|GetTimer)))))
        (:then_3
          ;[1 1 1] Makes manequinnes go back to their original positions
          (Utilities|FlowControl|DoOnce false :!label _label
            (:Completed
              (bind _outactors_2 (Actor|GetAllActorsOfClass "/Game/Sharan/Blueprints/RBP_Mannequine1.RBP_Mannequine1_C"))
              (for _array_element_2 _outactors_2
                (Default|TeleporttoStartPositionwithPoof _array_element_2)
                (Default|StopLogic _array_element_2))
              (goto _label Reset))))))))

(fn ConstructionScript)