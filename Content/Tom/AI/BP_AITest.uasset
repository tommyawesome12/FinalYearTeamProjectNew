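; Test AI Blueprint that can put its mesh into a random pose.
; On BeginPlay it casts player 0's character to BP_PlayerCharacter and caches it in PlayerRef.
; The SetPose event sets the mesh animation to a random entry from the Poses array; nothing in this file calls it.
; GetPlayerRef and GetThingFromPawn are empty stubs, and overlap and Tick are unimplemented.
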(event Custom|SetPose
  (bind _poses (Variables|Default|GetPoses))
  (Components|Animation|SetAnimation (Variables|Character|GetMesh) (Utilities|Array|Get(acopy) _poses (Math|Random|RandomIntegerinRange 0 (- (Utilities|Array|Length _poses) 1)))))

(event EventBeginPlay
  ;[1 1 1] Gets Player Reference
  (bind _asbp_player_character (Utilities|Casting|CastToBP_PlayerCharacter (Game|GetPlayerCharacter 0)))
  (Variables|Default|SetPlayerRef _asbp_player_character))

(event Collision|EventActorBeginOverlap
  (params (OtherActor :type Actor%20Object%20Reference)))

(event EventTick
  (params (DeltaSeconds :type Float%20%28single-precision%29)))

(fn ConstructionScript)

(fn GetPlayerRef
  (return 0))

(fn GetThingfromPawn
  (return 0))